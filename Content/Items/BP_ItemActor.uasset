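; BP_ItemActor is a world item pickup that the player interacts with to add it to their inventory.
; Interact passes the item ID and quantity from BPCItemData to the player's Inventory, then on success optionally adds a ProgressionManager flag, plays a sound and destroys the actor.
; LookAtActor returns the item's name from DT_ItemData_NEW.
; EndPlay replays the pickup sound for any reason, and the HasBeenPickedUp guard is never set true.
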(event EventEndPlay
  (params (EndPlayReason :type EEndPlayReason%20Enum :default "Destroyed"))
  ;[0.15 0.15 0.15 0.5] Sound
  (Audio|PlaySound2D (Variables|Default|GetS_PickupSound) 1.0 1.0 0.0 0 0))

(event EventInteractwith
  (params (Interactor :type Actor%20Object%20Reference))
  (bind _bpc_itemdata (Variables|Default|GetBPC_ItemData))
  ;[0.15 0.15 0.15 0.5] Interact event: when the player interacts, try to add this item to their InventoryComponent (via BPC_ItemData) and then play sound / destroy on success. The bHasBeenPickedUp guard prevents double-pickup. EndPlay-with-reason-Destroyed plays the pickup sound as a fallback.
  (if (not (Variables|Default|GetbHasBeenPickedUp))
    (bind _asbp_character_speltest_1 (Utilities|Casting|CastToBP_CharacterSpeltest1 (Game|GetPlayerCharacter 0)))
    (bind _returnvalue (Class|InventoryComponent|AddItemtoInventory (Variables|/Game/Grupp03_Test/Speltest1/BP_CharacterSpeltest1.BP_CharacterSpeltest1_C|GetInventory _asbp_character_speltest_1) (Variables|/Game/Blueprints/BP/InventoryCraftingBPs/BPC_ItemData.BPC_ItemData_C|GetItemID _bpc_itemdata) (Variables|/Game/Blueprints/BP/InventoryCraftingBPs/BPC_ItemData.BPC_ItemData_C|GetItemQuantity _bpc_itemdata)))
    (if _returnvalue
      ;[0.03689 0.02756 0.15 0.5] Progression Logic
      (if (Variables|/Game/Blueprints/BP/InventoryCraftingBPs/BPC_ItemData.BPC_ItemData_C|GetbAddProgressionFlagOnPickup (Variables|Default|GetBPC_ItemData))
        (bind _returnvalue_2 (Actor|GetActorOfClass "/Script/SPM_grupp3.ProgressionManager"))
        (Class|ProgressionManager|AddFlag _returnvalue_2 (Variables|/Game/Blueprints/BP/InventoryCraftingBPs/BPC_ItemData.BPC_ItemData_C|GetProgressionFlagOnPickup (Variables|Default|GetBPC_ItemData)))
        (Audio|PlaySound2D (Variables|Default|GetS_PickupSound) 1.0 1.0 0.0 0 0)
        (Actor|DestroyActor)
        (else
          ;[0.15 0.15 0.15 0.5] Sound
          (Audio|PlaySound2D (Variables|Default|GetS_PickupSound) 1.0 1.0 0.0 0 0)
          (Actor|DestroyActor)))
      (else
        (Variables|Default|SetbHasBeenPickedUp false)))))

(fn ConstructionScript)

(fn LookatActor
  (bind _returnvalue (Utilities|GetDataTableRow "/Game/DataTables/DT_ItemData_NEW.DT_ItemData_NEW" (Variables|/Game/Blueprints/BP/InventoryCraftingBPs/BPC_ItemData.BPC_ItemData_C|GetItemID (Variables|Default|GetBPC_ItemData)))
    (:then
      (return (.ItemName (Utilities|Struct|BreakItemDetail _returnvalue))))))