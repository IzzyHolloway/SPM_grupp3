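; BP_WaterLvl1 is an audio trigger actor, apparently for level 1 water ambience, that plays a sound when the player character enters its capsule.
; The construction script applies the configurable sound cue, ambience attenuation and capsule radius to its components.
; Each overlap by BP_ThirdPersonCharacter starts playback at a random offset within the cue's duration.
; The file has no logic to stop the sound on exit.
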(event OnComponentBeginOverlap(CapsuleCollider)
  (params (OverlappedComponent :type Primitive%20Component%20Object%20Reference) (OtherActor :type Actor%20Object%20Reference) (OtherComp :type Primitive%20Component%20Object%20Reference) (OtherBodyIndex :type Integer) (bFromSweep :type Boolean) (SweepResult :type Hit%20Result%20Structure%20%28by%20ref%29))
  (Utilities|Casting|CastToBP_ThirdPersonCharacter OtherActor)
  (Audio|Components|Audio|Play (Variables|Default|GetAudio) (Math|Random|RandomFloatinRange 0.0 (Variables|/Script/Engine.SoundBase|GetDuration (Variables|Default|GetSound%20Cue)))))

(event EventBeginPlay)

(event Collision|EventActorBeginOverlap
  (params (OtherActor :type Actor%20Object%20Reference)))

(event EventTick
  (params (DeltaSeconds :type Float%20%28single-precision%29)))

(fn ConstructionScript
  (Audio|Components|Audio|SetSound (Variables|Default|GetAudio) (Variables|Default|GetSound%20Cue))
  (Variables|/Script/Engine.AudioComponent|SetAttenuationSettings (Variables|Default|GetAudio) (Variables|Default|GetAmbianceSoundAttenuation))
  (Components|Capsule|SetCapsuleRadius (Variables|Default|GetCapsuleCollider) (Variables|Default|GetCapsuleRadius) true))