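; Pier actor that marks where the player can exit BP_Paula_Boat, with docking gated by story progression.
; When a boat enters ExitBoatTrigger, the pier checks a ProgressionManager flag, then either adds another flag and registers itself on the boat or refuses docking.
; Leaving the trigger clears the boat's pier reference.
; BeginPlay waits one tick to register boats already overlapping, without checking progression.
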(event OnComponentBeginOverlap(ExitBoatTrigger)
  (params (OverlappedComponent :type Primitive%20Component%20Object%20Reference) (OtherActor :type Actor%20Object%20Reference) (OtherComp :type Primitive%20Component%20Object%20Reference) (OtherBodyIndex :type Integer) (bFromSweep :type Boolean) (SweepResult :type Hit%20Result%20Structure%20%28by%20ref%29))
  ;[0.15 0.15 0.15 0.5] Check if the overlapping actor is the boat. If yes, cast it to the boat class
  (if (Utilities|ClassIsChildOf (Utilities|GetClass OtherActor) "/Game/Grupp03_Test/Paula/BP_Paula_Boat.BP_Paula_Boat_C")
    (bind _asbp_paula_boat (Utilities|Casting|CastToBP_Paula_Boat OtherActor))
    (Development|PrintString "Press E to exit the boat" true true "(R=0.000000,G=0.660000,B=1.000000,A=1.000000)" 3.0)
    ;[0.15 0.15 0.15 0.5] Enable pressing E and hopping out of boat in Boat class
    (Variables|/Game/Grupp03_Test/Paula/BP_Paula_Boat.BP_Paula_Boat_C|SetLookingAtPier _asbp_paula_boat true)
    ;;[0 0.08424 0.15 0.5] Progression Flag added after solving Intro Puzzle and jumping off at Island1
    (bind _returnvalue (Actor|GetActorOfClass "/Script/SPM_grupp3.ProgressionManager"))
    (if (Class|ProgressionManager|HasFlag _returnvalue (Variables|Default|GetHasFlag))
      (Class|ProgressionManager|AddFlag _returnvalue (Variables|Default|GetAddingFlag))
      (Variables|/Game/Grupp03_Test/Paula/BP_Paula_Boat.BP_Paula_Boat_C|SetPierLookedAt _asbp_paula_boat self)
      (else
        (Development|PrintString "Catn't dock here")
        (Variables|/Game/Grupp03_Test/Paula/BP_Paula_Boat.BP_Paula_Boat_C|SetLookingAtPier _asbp_paula_boat false)))))

(event OnComponentEndOverlap(ExitBoatTrigger)
  (params (OverlappedComponent :type Primitive%20Component%20Object%20Reference) (OtherActor :type Actor%20Object%20Reference) (OtherComp :type Primitive%20Component%20Object%20Reference) (OtherBodyIndex :type Integer))
  ;[0.15 0.15 0.15 0.5] Check if the overlapping actor is the boat. If yes, cast it to the boat class
  (if (Utilities|ClassIsChildOf (Utilities|GetClass OtherActor) "/Game/Grupp03_Test/Paula/BP_Paula_Boat.BP_Paula_Boat_C")
    (bind _asbp_paula_boat (Utilities|Casting|CastToBP_Paula_Boat OtherActor))
    ;[0.15 0.15 0.15 0.5] Disable pressing E and hopping out of boat in Boat class
    (Variables|/Game/Grupp03_Test/Paula/BP_Paula_Boat.BP_Paula_Boat_C|SetLookingAtPier _asbp_paula_boat false)
    (Variables|/Game/Grupp03_Test/Paula/BP_Paula_Boat.BP_Paula_Boat_C|SetPierLookedAt _asbp_paula_boat 0)))

(event EventBeginPlay
  ;[0.15 0.15 0.15 0.5] Check if boat is already in the trigger zone for exiting the boat
  ;;[0.15 0.15 0.15 0.5] At BeginPlay, the engine hasn't checked for overlapping actors yet
  (Utilities|FlowControl|DelayUntilNextTick)
  (for _array_element (Collision|GetOverlappingActors (Variables|Default|GetExitBoatTrigger) "/Game/Grupp03_Test/Paula/BP_Paula_Boat.BP_Paula_Boat_C" :!class /Script/Engine.PrimitiveComponent)
    (bind _asbp_paula_boat (Utilities|Casting|CastToBP_Paula_Boat _array_element))
    ;[0.15 0.15 0.15 0.5] Enable pressing E and hopping out of boat in Boat class
    (Variables|/Game/Grupp03_Test/Paula/BP_Paula_Boat.BP_Paula_Boat_C|SetLookingAtPier _asbp_paula_boat true)
    (Variables|/Game/Grupp03_Test/Paula/BP_Paula_Boat.BP_Paula_Boat_C|SetPierLookedAt _asbp_paula_boat self)))

(event Collision|EventActorBeginOverlap
  (params (OtherActor :type Actor%20Object%20Reference)))

(event EventTick
  (params (DeltaSeconds :type Float%20%28single-precision%29)))

(fn ConstructionScript)