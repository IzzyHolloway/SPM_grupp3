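; BP_NPCInteractable_Island2 is a test NPC actor that walks along a spline path taken from a referenced SplineActor.
; The construction script caches that actor's Spline component, and a debug O key sets IsWalking.
; While walking, Tick advances distance by Speed, moves the NPC to that world-space spline point, and stops at the spline's end.
; Rotation along the tangent is left unwired because the NPC looks identical from all sides.
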(event EventBeginPlay
  ;[0.15 0.15 0.15 0.5] Only for testing: Trigger walking when pressing a debug key
  (Input|EnableInput (Game|GetPlayerController 0)))

(event Collision|EventActorBeginOverlap
  (params (OtherActor :type Actor%20Object%20Reference)))

(event EventTick
  (params (DeltaSeconds :type Float%20%28single-precision%29))
  (if (Variables|Default|GetIsWalking)
    ;[0.15 0.15 0.15 0.5] Update current distance: Add distance walked this frame
    (Variables|Default|SetCurrentDistance (+ (Variables|Default|GetCurrentDistance) (* (Variables|Default|GetSpeed) DeltaSeconds)))
    ;[0.15 0.15 0.15 0.5] Set new actor location: distance along spline
    (Transformation|SetActorLocation (Spline|GetLocationatDistanceAlongSpline (Variables|Default|GetSpline) (Variables|Default|GetCurrentDistance) "World") false false)
    ;[0.15 0.15 0.15 0.5] End walking if whole distances has been travelled
    (if (>= (Variables|Default|GetCurrentDistance) (Spline|GetSplineLength (Variables|Default|GetSpline)))
      (Variables|Default|SetIsWalking false))))

(event Input|KeyboardEvents|O
  (params (Key :type Key%20Structure :default "None"))
  ;[0.15 0.15 0.15 0.5] Only for debugging: Trigger walking when pressing debug key
  (:Pressed
    ;[0.15 0.15 0.15 0.5] Start walking
    (Variables|Default|SetIsWalking true)))

(fn ConstructionScript
  (Variables|Default|SetSpline (Actor|GetComponentbyClass (Variables|Default|GetSplineActor) "/Script/Engine.SplineComponent")))