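; Boat pawn that the player possesses, handling its engine audio, lantern visibility and camera hand-off.
; A looping timer polls ProgressionManager's LitLantern flag to show or hide the lantern and lights.
; While possessed, Tick feeds speed into the BoatSound parameter and starts audio once on movement, re-armed by BoatSoundStop.
; Custom events move BP_CameraDirector to an exit camera, restore it as view target, shake the camera and toggle input.
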(event Custom|UpdateLanternVisibility
  (bind _returnvalue (Actor|GetActorOfClass "/Script/SPM_grupp3.ProgressionManager"))
  (if (Class|ProgressionManager|HasFlag _returnvalue "LitLantern")
    (Rendering|SetVisibility (Variables|Default|GetLantern) true true)
    (Rendering|SetVisibility (Variables|Default|GetLanternLight) true true)
    (Rendering|SetVisibility (Variables|Default|GetPointLight) true true)
    (else
      (Rendering|SetVisibility (Variables|Default|GetLantern) false false)
      (Rendering|SetVisibility (Variables|Default|GetLanternLight) false false)
      (Rendering|SetVisibility (Variables|Default|GetPointLight) false false))))

(event Custom|ResetBoatAudio
  ;[0.15 0.15 0.15 0.5] boatSound - start
  (Utilities|FlowControl|DoOnce false) ; enters at Reset
)

(event Custom|Camera%20Shake
  (Camera|PlayWorldCameraShake "/Game/Grupp03_Test/Madde/MaddeBlueprints/BP_CamShake.BP_CamShake_C" (Transformation|GetActorLocation) 0.0 1e+03))

(event Custom|Stop%20Boat%20Movement
  (Input|DisableInput self (Game|GetPlayerController 0)))

(event Custom|Start%20Boat%20Movement
  (Input|EnableInput self (Game|GetPlayerController 0)))

(event EventTick
  (params (DeltaSeconds :type Float%20%28single-precision%29))
  (bind _returnvalue (Transformation|GetVelocity))
  (bind _returnvalue_2 (Math|Vector|VectorLength _returnvalue))
  ;[0.15 0.15 0.15 0.5] boatSound - start
  (if (Variables|Default|GetPossessed)
    (Class|FMODAudioComponent|SetParameter (Variables|Default|GetBoat) "BoatSound" _returnvalue_2)
    (if (not (Math|Float|NearlyEqual(Float) _returnvalue_2 0.0 5.0))
      (Utilities|FlowControl|DoOnce false
        (:Completed
          (Class|FMODBlueprintStatics|PlayEvent2D "/Game/FMOD/Events/StartBoat.StartBoat")
          (Class|FMODAudioComponent|Play (Variables|Default|GetBoat)))))))

(event Collision|EventActorBeginOverlap
  (params (OtherActor :type Actor%20Object%20Reference)))

(event EventFixCameraAfterRepossessingPlayer
  ;[0.15 0.15 0.15 0.5] Fix camera after repossessing character
  (bind _returnvalue (Actor|GetActorOfClass "/Game/Grupp03_Test/Madde/MaddeBlueprints/BP_CameraDirector.BP_CameraDirector_C"))
  (Game|Player|SetViewTargetwithBlend 0 _returnvalue 0.0 "VTBlend_Linear" 0.0 false))

(event EventBoatSoundStop
  ;[0.15 0.15 0.15 0.5] BoatSound-stop
  (Class|FMODAudioComponent|Stop (Variables|Default|GetBoat))
  (CallFunction|ResetBoatAudio))

(event EventBeginPlay
  (Variables|Default|SetPossessed false)
  (Utilities|Time|SetTimerbyEvent (delegate Custom|UpdateLanternVisibility) 0.2 true))

(event EventPossessed
  (params (NewController :type Controller%20Object%20Reference))
  (Variables|Default|SetPossessed true))

(event EventUnpossessed
  (params (OldController :type Controller%20Object%20Reference))
  (Variables|Default|SetPossessed false))

(event EventSetCameraPositionwhenExiting
  (params (CameraComponent :type Cine%20Camera%20Component%20Object%20Reference))
  (bind _returnvalue (Actor|GetActorOfClass "/Game/Grupp03_Test/Madde/MaddeBlueprints/BP_CameraDirector.BP_CameraDirector_C"))
  (Transformation|SetWorldLocation (Variables|/Script/Engine.Actor|GetRootComponent _returnvalue) (Transformation|GetWorldLocation CameraComponent) false false)
  (Transformation|SetWorldRotation (Variables|/Script/Engine.Actor|GetRootComponent _returnvalue) (Transformation|GetWorldRotation CameraComponent) false false))

(fn ConstructionScript)