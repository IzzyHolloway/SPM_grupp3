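; Drivable boat pawn that the player boards and exits at piers, moving along its forward axis with yaw-only look.
; Its trigger offers boarding to the character, gated by a ProgressionManager flag.
; Exiting, when LookingAtPier is set, moves the attached character onto the pier, repossesses it and hands the view to BP_CameraDirector at the boat camera's transform.
; Tick feeds speed to boat audio, starting it once per ride.
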(event OnComponentBeginOverlap(EnterTrigger)
  (params (OverlappedComponent :type Primitive%20Component%20Object%20Reference) (OtherActor :type Actor%20Object%20Reference) (OtherComp :type Primitive%20Component%20Object%20Reference) (OtherBodyIndex :type Integer) (bFromSweep :type Boolean) (SweepResult :type Hit%20Result%20Structure%20%28by%20ref%29))
  ;[0.15 0.15 0.15 0.5] Check if the overlapping object is the player. If yes, cast it to the Character class
  (if (Utilities|ClassIsChildOf (Utilities|GetClass OtherActor) "/Game/Grupp03_Test/Speltest1/BP_CharacterSpeltest1.BP_CharacterSpeltest1_C")
    (bind _asbp_character_speltest_1 (Utilities|Casting|CastToBP_CharacterSpeltest1 OtherActor))
    ;[0.15 0.15 0.15 0.5] Enable pressing E and hopping in in Character class
    (Variables|/Game/Grupp03_Test/Speltest1/BP_CharacterSpeltest1.BP_CharacterSpeltest1_C|SetLookingAtBoat _asbp_character_speltest_1 true)
    ;;[0 0.1055 0.15 0.5] Addding progression flags, checking if the player is ready to board
    (bind _returnvalue (Actor|GetActorOfClass "/Script/SPM_grupp3.ProgressionManager"))
    (if (Class|ProgressionManager|HasFlag _returnvalue "HomeReadyForBoat")
      (Class|ProgressionManager|AddFlag _returnvalue "EnteredBoat")
      (Variables|/Game/Grupp03_Test/Speltest1/BP_CharacterSpeltest1.BP_CharacterSpeltest1_C|SetBoatLookedAt _asbp_character_speltest_1 self)
      (else
        (Variables|/Game/Grupp03_Test/Speltest1/BP_CharacterSpeltest1.BP_CharacterSpeltest1_C|SetLookingAtBoat _asbp_character_speltest_1 false)))))

(event OnComponentEndOverlap(EnterTrigger)
  (params (OverlappedComponent :type Primitive%20Component%20Object%20Reference) (OtherActor :type Actor%20Object%20Reference) (OtherComp :type Primitive%20Component%20Object%20Reference) (OtherBodyIndex :type Integer))
  ;[0.15 0.15 0.15 0.5] Check if the overlapping object is the player. If yes, cast it to the Character class
  (if (Utilities|ClassIsChildOf (Utilities|GetClass OtherActor) "/Game/Grupp03_Test/Speltest1/BP_CharacterSpeltest1.BP_CharacterSpeltest1_C")
    (bind _asbp_character_speltest_1 (Utilities|Casting|CastToBP_CharacterSpeltest1 OtherActor))
    ;[0.15 0.15 0.15 0.5] Disable pressing E and hopping in in Character class
    (Variables|/Game/Grupp03_Test/Speltest1/BP_CharacterSpeltest1.BP_CharacterSpeltest1_C|SetLookingAtBoat _asbp_character_speltest_1 false)
    (Variables|/Game/Grupp03_Test/Speltest1/BP_CharacterSpeltest1.BP_CharacterSpeltest1_C|SetBoatLookedAt _asbp_character_speltest_1 0)))

(event Custom|ResetBoatAudio
  ;[0.15 0.15 0.15 0.5] boatSound - start
  (Utilities|FlowControl|DoOnce false) ; enters at Reset
)

(event Input|EnhancedActionEvents|EnhancedInputActionIA_Move
  (params (ActionValue :type Vector%202D%20Structure) (ElapsedSeconds :type Float%20%28double-precision%29) (TriggeredSeconds :type Float%20%28double-precision%29) (InputAction :type Input%20Action%20Object%20Reference :default "/Game/Input/Actions/IA_Move.IA_Move"))
  (Pawn|Input|AddMovementInput (Transformation|GetActorForwardVector) (.y ActionValue) false))

(event Input|EnhancedActionEvents|EnhancedInputActionIA_Look
  (params (ActionValue :type Vector%202D%20Structure) (ElapsedSeconds :type Float%20%28double-precision%29) (TriggeredSeconds :type Float%20%28double-precision%29) (InputAction :type Input%20Action%20Object%20Reference :default "/Game/Input/Actions/IA_Look.IA_Look"))
  (Pawn|Input|AddControllerYawInput (.x ActionValue)))

(event Input|EnhancedActionEvents|EnhancedInputActionIA_MouseLook
  (params (ActionValue :type Vector%202D%20Structure) (ElapsedSeconds :type Float%20%28double-precision%29) (TriggeredSeconds :type Float%20%28double-precision%29) (InputAction :type Input%20Action%20Object%20Reference :default "/Game/Input/Actions/IA_MouseLook.IA_MouseLook"))
  (Pawn|Input|AddControllerYawInput (.x ActionValue)))

(event EventTick
  (params (DeltaSeconds :type Float%20%28single-precision%29))
  (bind _returnvalue (Transformation|GetVelocity))
  (bind _returnvalue_2 (Math|Vector|VectorLength _returnvalue))
  ;[0.15 0.15 0.15 0.5] boatSound - start
  (if (Variables|Default|GetPossessed)
    (Class|FMODAudioComponent|SetParameter (Variables|Default|GetBoat) "BoatSound" _returnvalue_2)
    (if (not (Math|Float|NearlyEqual(Float) _returnvalue_2 0.0 5.0))
      (Utilities|FlowControl|DoOnce false
        (:Completed
          (Class|FMODBlueprintStatics|PlayEvent2D "/Game/FMOD/Events/StartBoat.StartBoat")
          (Class|FMODAudioComponent|Play (Variables|Default|GetBoat)))))))

(event Collision|EventActorBeginOverlap
  (params (OtherActor :type Actor%20Object%20Reference)))

(event EventBeginPlay
  (Variables|Default|SetPossessed false))

(event EventPossessed
  (params (NewController :type Controller%20Object%20Reference))
  (Variables|Default|SetPossessed true))

(event EventUnpossessed
  (params (OldController :type Controller%20Object%20Reference))
  (Variables|Default|SetPossessed false))

(event Input|GamepadEvents|GamepadFaceButtonLeft
  (params (Key :type Key%20Structure))
  (bind _returnvalue (Game|GetPlayerController 0))
  (bind _pierlookedat (Variables|Default|GetPierLookedAt))
  (bind _camera (Variables|Default|GetCamera))
  (:Pressed
    ;[0.15 0.15 0.15 0.5] Make sure we're in reach of a pier
    (if (Variables|Default|GetLookingAtPier)
      (bind _returnvalue_2 (Actor|GetActorOfClass "/Game/Grupp03_Test/Madde/Blueprints/BP_CameraDirector.BP_CameraDirector_C"))
      (Transformation|SetWorldLocation (Variables|/Script/Engine.Actor|GetRootComponent _returnvalue_2) (Transformation|GetWorldLocation _camera) false false)
      (Transformation|SetWorldRotation (Variables|/Script/Engine.Actor|GetRootComponent _returnvalue_2) (Transformation|GetWorldRotation _camera) false false)
      ;[0.15 0.15 0.15 0.5] Find the Player Character among the children
      (for _array_element (Actor|GetAttachedActors true false)
        (if (Utilities|ClassIsChildOf (Utilities|GetClass _array_element) "/Game/Grupp03_Test/Speltest1/BP_CharacterSpeltest1.BP_CharacterSpeltest1_C")
          (bind _asbp_character_speltest_1 (Utilities|Casting|CastToBP_CharacterSpeltest1 _array_element))
          ;[0.15 0.15 0.15 0.5] Detach Player Character
          (Transformation|DetachFromActor _asbp_character_speltest_1 "KeepRelative" "KeepRelative" "KeepRelative")
          ;[0.15 0.15 0.15 0.5] Move Player on top of the pier
          (Transformation|SetActorLocation _asbp_character_speltest_1 (+ (Transformation|GetActorLocation _pierlookedat) (Variables|/Game/Grupp03_Test/Paula/BP_Paula_Pier.BP_Paula_Pier_C|GetCharacterSpawnOffset _pierlookedat)) false false)
          ;[0.15 0.15 0.15 0.5] Repossess player character
          (Pawn|Possess _returnvalue _asbp_character_speltest_1)
          ;[0.15 0.15 0.15 0.5] Fix camera after repossessing character
          (bind _returnvalue_3 (Actor|GetActorOfClass "/Game/Grupp03_Test/Madde/Blueprints/BP_CameraDirector.BP_CameraDirector_C"))
          (Game|Player|SetViewTargetwithBlend _returnvalue _returnvalue_3 0.0 "VTBlend_Linear" 0.0 false)
          ;[0.15 0.15 0.15 0.5] BoatSound-stop
          (Class|FMODAudioComponent|Stop (Variables|Default|GetBoat))
          (CallFunction|ResetBoatAudio))))))

(event Input|KeyboardEvents|E
  (params (Key :type Key%20Structure))
  (bind _returnvalue (Game|GetPlayerController 0))
  (bind _pierlookedat (Variables|Default|GetPierLookedAt))
  (bind _camera (Variables|Default|GetCamera))
  ;[0.15 0.15 0.15 0.5] Player wants to exit the boat
  (:Pressed
    ;[0.15 0.15 0.15 0.5] Make sure we're in reach of a pier
    (if (Variables|Default|GetLookingAtPier)
      (bind _returnvalue_2 (Actor|GetActorOfClass "/Game/Grupp03_Test/Madde/Blueprints/BP_CameraDirector.BP_CameraDirector_C"))
      (Transformation|SetWorldLocation (Variables|/Script/Engine.Actor|GetRootComponent _returnvalue_2) (Transformation|GetWorldLocation _camera) false false)
      (Transformation|SetWorldRotation (Variables|/Script/Engine.Actor|GetRootComponent _returnvalue_2) (Transformation|GetWorldRotation _camera) false false)
      ;[0.15 0.15 0.15 0.5] Find the Player Character among the children
      (for _array_element (Actor|GetAttachedActors true false)
        (if (Utilities|ClassIsChildOf (Utilities|GetClass _array_element) "/Game/Grupp03_Test/Speltest1/BP_CharacterSpeltest1.BP_CharacterSpeltest1_C")
          (bind _asbp_character_speltest_1 (Utilities|Casting|CastToBP_CharacterSpeltest1 _array_element))
          ;[0.15 0.15 0.15 0.5] Detach Player Character
          (Transformation|DetachFromActor _asbp_character_speltest_1 "KeepRelative" "KeepRelative" "KeepRelative")
          ;[0.15 0.15 0.15 0.5] Move Player on top of the pier
          (Transformation|SetActorLocation _asbp_character_speltest_1 (+ (Transformation|GetActorLocation _pierlookedat) (Variables|/Game/Grupp03_Test/Paula/BP_Paula_Pier.BP_Paula_Pier_C|GetCharacterSpawnOffset _pierlookedat)) false false)
          ;[0.15 0.15 0.15 0.5] Repossess player character
          (Pawn|Possess _returnvalue _asbp_character_speltest_1)
          ;[0.15 0.15 0.15 0.5] Fix camera after repossessing character
          (bind _returnvalue_3 (Actor|GetActorOfClass "/Game/Grupp03_Test/Madde/Blueprints/BP_CameraDirector.BP_CameraDirector_C"))
          (Game|Player|SetViewTargetwithBlend _returnvalue _returnvalue_3 0.0 "VTBlend_Linear" 0.0 false)
          ;[0.15 0.15 0.15 0.5] BoatSound-stop
          (Class|FMODAudioComponent|Stop (Variables|Default|GetBoat))
          (CallFunction|ResetBoatAudio))))))

(fn ConstructionScript)