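; Drivable boat pawn with sprint boost, engine audio, wake particles and a tutorial widget shown on first player possession.
; Boost drains and recharges on looping timers; emptying it starts a cooldown and calls the water AI's hit event.
; Tick starts audio and switches particles from speed and heading, while a polling timer lights the lantern from a ProgressionManager flag.
; Helper events handle camera shake, input locking and camera-director handoff on exit.
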(event Custom|UpdateLanternVisibility
  (bind _returnvalue (Actor|GetActorOfClass "/Script/SPM_grupp3.ProgressionManager"))
  (if (Class|ProgressionManager|HasFlag _returnvalue "LitLantern")
    (Utilities|FlowControl|Delay 0.75)
    (Utilities|FlowControl|DoOnce false
      (:Completed
        (Audio|PlaySound2D 0 1.0 1.0 0.0 0 0)
        (Rendering|SetVisibility (Variables|Default|GetLantern) true true)
        (Rendering|SetVisibility (Variables|Default|GetSpotLight) true true)
        (Rendering|SetVisibility (Variables|Default|GetPointLight) true true)))
    (else
      (Rendering|SetVisibility (Variables|Default|GetLantern) false false)
      (Rendering|SetVisibility (Variables|Default|GetSpotLight) false false)
      (Rendering|SetVisibility (Variables|Default|GetPointLight) false false))))

(event Custom|ResetBoatAudio
  ;[0.15 0.15 0.15 0.5] boatSound - start
  (Utilities|FlowControl|DoOnce false) ; enters at Reset
)

(event Custom|Camera%20Shake
  ;[0.15 0.15 0.15 0.5] Camera shake for water AI
  (Camera|PlayWorldCameraShake "/Game/Grupp03_Test/Madde/Blueprints/BP_CamShake.BP_CamShake_C" (Transformation|GetActorLocation) 0.0 1e+03))

(event Custom|Stop%20Boat%20Movement
  (Input|DisableInput self (Game|GetPlayerController 0)))

(event Custom|Start%20Boat%20Movement
  (Input|EnableInput self (Game|GetPlayerController 0)))

(event Custom|Drain%20Boost
  ;[0.15 0.15 0.15 0.5] Boost functionality
  (bind _output_get (Variables|Default|SetBoostResource (- (Variables|Default|GetBoostResource) 0.05)))
  (if (<= _output_get 0.0)
    (Utilities|Time|ClearandInvalidateTimerbyHandle (Variables|Default|GetBoostTimeHandler))
    (Variables|Default|SetbIsBoostOnCooldown true)
    (Class|BoatFunctionality|StopSprint)
    (Components|Activation|Deactivate (Variables|Default|GetBoatBoostParticles))
    (bind _returnvalue (Actor|GetActorOfClass "/Game/Grupp03_Test/Madde/Blueprints/BP_WaterAI.BP_WaterAI_C"))
    (Default|AIHitEvent _returnvalue)))

(event Custom|Recharge%20Boost
  ;[0.15 0.15 0.15 0.5] Boost functionality
  (bind _output_get (Variables|Default|SetBoostResource (+ (Variables|Default|GetBoostResource) 0.1)))
  (if (>= _output_get (Variables|Default|GetMaxBoostResource))
    (Utilities|Time|ClearandInvalidateTimerbyHandle (Variables|Default|GetRechardTimeHandler))
    (Variables|Default|SetbIsBoostOnCooldown false)
    (else
      (Development|PrintString "Cant boost!")
      (Components|Activation|Deactivate (Variables|Default|GetBoatBoostParticles)))))

(event Input|EnhancedActionEvents|EnhancedInputActionIA_Sprint
  (params (ActionValue :type Boolean) (ElapsedSeconds :type Float%20%28double-precision%29) (TriggeredSeconds :type Float%20%28double-precision%29) (InputAction :type Input%20Action%20Object%20Reference :default "/Game/Input/Actions/IA_Sprint.IA_Sprint"))
  (bind _movementcomponent (Variables|Default|GetMovementComponent))
  (bind _velocity (Variables|/Script/Engine.MovementComponent|GetVelocity _movementcomponent))
  ;[0.15 0.15 0.15 0.5] Boost functionality
  (:Triggered
    (if (and (> (Math|Vector|VectorLength _velocity) 6e+02) (> (Math|Vector|DotProduct _velocity (Math|Vector|GetForwardVector (Variables|Default|GetBoat))) 0.0))
      (if (not (Variables|Default|GetbIsBoostOnCooldown))
        (Components|Activation|Activate (Variables|Default|GetBoatBoostParticles) false)
        (Components|Activation|Deactivate (Variables|Default|GetBoatParticles)))
      (else
        (Components|Activation|Deactivate (Variables|Default|GetBoatBoostParticles)))))
  (:Started
    (if (Variables|Default|GetbIsBoostOnCooldown)
      (if (not (Variables|Default|GetbHasWidgetOnScreen))
        (Variables|Default|SetbHasWidgetOnScreen true)
        (bind _returnvalue (UserInterface|CreateWidget "/Game/Grupp03_Test/Madde/Widgets/WBP_NoMoreBoost.WBP_NoMoreBoost_C"))
        (UserInterface|Viewport|AddtoViewport _returnvalue 0)
        (Utilities|FlowControl|Delay 2.0)
        (Widget|RemovefromParent _returnvalue)
        (Variables|Default|SetbHasWidgetOnScreen false)
        (Components|Activation|Deactivate (Variables|Default|GetBoatBoostParticles)))
      (elif (> (Variables|Default|GetBoostResource) 0.0)
        (Utilities|Time|ClearandInvalidateTimerbyHandle (Variables|Default|GetRechardTimeHandler))
        (bind _returnvalue_2 (Utilities|Time|SetTimerbyEvent (delegate Custom|Drain%20Boost) 0.05 true))
        (Variables|Default|SetBoostTimeHandler _returnvalue_2)
        (Variables|Default|SetbIsBoosting true)
        (Class|BoatFunctionality|StartSprint))))
  (:Completed
    (Utilities|Time|ClearandInvalidateTimerbyHandle (Variables|Default|GetBoostTimeHandler))
    (bind _returnvalue_3 (Utilities|Time|SetTimerbyEvent (delegate Custom|Recharge%20Boost) 0.1 true))
    (Variables|Default|SetRechardTimeHandler _returnvalue_3)
    (Variables|Default|SetbIsBoosting false)
    (Class|BoatFunctionality|StopSprint)
    (Components|Activation|Deactivate (Variables|Default|GetBoatBoostParticles))))

(event EventTick
  (params (DeltaSeconds :type Float%20%28single-precision%29))
  (bind _movementcomponent (Variables|Default|GetMovementComponent))
  (bind _boatparticles (Variables|Default|GetBoatParticles))
  (bind _velocity (Variables|/Script/Engine.MovementComponent|GetVelocity _movementcomponent))
  (bind _returnvalue (Math|Vector|VectorLength _velocity))
  (Utilities|FlowControl|Sequence
    (:then_0
      ;[0.15 0.15 0.15 0.5] boatSound - start
      (if (Variables|Default|GetPossessed)
        (if (not (Math|Float|NearlyEqual(Float) (Math|Vector|VectorLength (Transformation|GetVelocity)) 0.0 5.0))
          (Utilities|FlowControl|DoOnce false
            (:Completed
              (Class|FMODBlueprintStatics|PlayEvent2D "/Game/FMOD/Events/StartBoat.StartBoat")
              (Class|FMODAudioComponent|Play (Variables|Default|GetBoat)))))))
    (:then_1
      ;[0.15 0.15 0.15 0.5] Make sure rendering happens fully
      (Class|PlayerCameraManager|SetGameCameraCutThisFrame (Variables|/Script/Engine.PlayerController|GetPlayerCameraManager (Game|GetPlayerController 0))))
    (:then_2
      ;[0.15 0.15 0.15 0.5] Adding particles when you drive the boat
      (if (and (> (Math|Vector|DotProduct _velocity (Math|Vector|GetForwardVector (Variables|Default|GetBoat))) 0.0) (> _returnvalue 3e+02))
        (if (< _returnvalue 1.5e+03)
          (if (Variables|Default|GetPossessed)
            (Components|Activation|Activate _boatparticles false)
            (else
              (Components|Activation|Deactivate _boatparticles :!label _label)
              (Components|Activation|Deactivate (Variables|Default|GetBoatBoostParticles)))))
        (else
          (goto _label))))))

(event Collision|EventActorBeginOverlap
  (params (OtherActor :type Actor%20Object%20Reference)))

(event EventFixCameraAfterRepossessingPlayer
  ;[0.15 0.15 0.15 0.5] Fix camera after repossessing character
  (bind _returnvalue (Actor|GetActorOfClass "/Game/Grupp03_Test/Madde/Blueprints/BP_CameraDirector.BP_CameraDirector_C"))
  (Game|Player|SetViewTargetwithBlend 0 _returnvalue 0.0 "VTBlend_Linear" 0.0 false))

(event EventBoatSoundStop
  ;[0.15 0.15 0.15 0.5] BoatSound-stop
  (Class|FMODAudioComponent|Stop (Variables|Default|GetBoat))
  (CallFunction|ResetBoatAudio))

(event EventBeginPlay
  (Variables|Default|SetPossessed false)
  (Utilities|Time|SetTimerbyEvent (delegate Custom|UpdateLanternVisibility) 0.2 true))

(event EventUnpossessed
  (params (OldController :type Controller%20Object%20Reference))
  (Variables|Default|SetPossessed false))

(event EventPossessed
  (params (NewController :type Controller%20Object%20Reference))
  ;[1 0.3591 0.7674 0.5] Widget BoatTutorial function
  (Variables|Default|SetPossessed true)
  (if (Class|Controller|IsPlayerController NewController)
    (Utilities|FlowControl|DoOnce false
      (:Completed
        (if (not (Variables|Default|GetHas%20Shown%20Tutorial))
          (Variables|Default|SetHas%20Shown%20Tutorial false)
          (bind _returnvalue (UserInterface|CreateWidget "/Game/Grupp03_Test/Izzy/WB_BoatTutorial.WB_BoatTutorial_C"))
          (UserInterface|Viewport|AddtoViewport _returnvalue 0)
          (Default|ShowBoatTutorial _returnvalue))))))

(event EventSetCameraPositionwhenExiting
  (params (CameraComponent :type Cine%20Camera%20Component%20Object%20Reference))
  (bind _returnvalue (Actor|GetActorOfClass "/Game/Grupp03_Test/Madde/Blueprints/BP_CameraDirector.BP_CameraDirector_C"))
  (Transformation|SetWorldLocation (Variables|/Script/Engine.Actor|GetRootComponent _returnvalue) (Transformation|GetWorldLocation CameraComponent) false false)
  (Transformation|SetWorldRotation (Variables|/Script/Engine.Actor|GetRootComponent _returnvalue) (Transformation|GetWorldRotation CameraComponent) false false))

(fn ConstructionScript)