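; Pier actor whose trigger lets the player's boat register it as a place to exit.
; Trigger overlaps set or clear the pier in reach on BoatFunctionality; BeginPlay checks one tick late for boats already inside.
; Entering shows an exit prompt and, if ProgressionManager has the required flag, adds another; otherwise it prints a can't-dock message.
; The pier is registered even when that flag is missing.
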(event OnComponentBeginOverlap(ExitBoatTrigger)
  (params (OverlappedComponent :type Primitive%20Component%20Object%20Reference) (OtherActor :type Actor%20Object%20Reference) (OtherComp :type Primitive%20Component%20Object%20Reference) (OtherBodyIndex :type Integer) (bFromSweep :type Boolean) (SweepResult :type Hit%20Result%20Structure%20%28by%20ref%29))
  ;[0.15 0.15 0.15 0.5] Check if the overlapping actor is the boat. If yes, cast it to the boat class
  (if (Utilities|ClassIsChildOf (Utilities|GetClass OtherActor) "/Script/SPM_grupp3.BoatFunctionality")
    (bind _asboat_functionality (Utilities|Casting|CastToBoatFunctionality OtherActor))
    (Development|PrintString "Press E to exit the boat" true true "(R=0.000000,G=0.660000,B=1.000000,A=1.000000)" 3.0)
    ;[0.15 0.15 0.15 0.5] Enable pressing E and hopping out of boat in Boat class
    ;;[0 0.08424 0.15 0.5] Progression Flag added after solving Intro Puzzle and jumping off at Island1
    (bind _returnvalue (Actor|GetActorOfClass "/Script/SPM_grupp3.ProgressionManager"))
    (if (Class|ProgressionManager|HasFlag _returnvalue (Variables|Default|GetHasFlag))
      (Class|ProgressionManager|AddFlag _returnvalue (Variables|Default|GetAddingFlag))
      (else
        (Development|PrintString "Catn't dock here")))
    (Class|BoatFunctionality|SetPierinReach _asboat_functionality self)))

(event OnComponentEndOverlap(ExitBoatTrigger)
  (params (OverlappedComponent :type Primitive%20Component%20Object%20Reference) (OtherActor :type Actor%20Object%20Reference) (OtherComp :type Primitive%20Component%20Object%20Reference) (OtherBodyIndex :type Integer))
  ;[0.15 0.15 0.15 0.5] Check if the overlapping actor is the boat. If yes, cast it to the boat class
  (if (Utilities|ClassIsChildOf (Utilities|GetClass OtherActor) "/Script/SPM_grupp3.BoatFunctionality")
    (bind _asboat_functionality (Utilities|Casting|CastToBoatFunctionality OtherActor))
    ;[0.15 0.15 0.15 0.5] Disable pressing E and hopping out of boat in Boat class
    (Class|BoatFunctionality|RemovePierinReach _asboat_functionality)))

(event EventBeginPlay
  ;[0.15 0.15 0.15 0.5] Check if boat is already in the trigger zone for exiting the boat
  ;;[0.15 0.15 0.15 0.5] At BeginPlay, the engine hasn't checked for overlapping actors yet
  (Utilities|FlowControl|DelayUntilNextTick)
  (for _array_element (Collision|GetOverlappingActors (Variables|Default|GetExitBoatTrigger) "/Script/SPM_grupp3.BoatFunctionality" :!class /Script/Engine.PrimitiveComponent)
    (bind _asboat_functionality (Utilities|Casting|CastToBoatFunctionality _array_element))
    ;[0.15 0.15 0.15 0.5] Enable pressing E and hopping out of boat in Boat class
    (Class|BoatFunctionality|SetPierinReach _asboat_functionality self)))

(event Collision|EventActorBeginOverlap
  (params (OtherActor :type Actor%20Object%20Reference)))

(event EventTick
  (params (DeltaSeconds :type Float%20%28single-precision%29)))

(fn ConstructionScript)