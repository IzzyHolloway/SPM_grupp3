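; Level 2 trigger actor that plays the opening cutscene once when its box is overlapped, with hold-to-skip support.
; On overlap it enables input, then creates the cutscene and skip prompt widgets and starts the media player.
; Dialogue-advance and skip inputs start or stop the prompt's hold.
; A completed hold or a fixed delay matching the video length calls a guarded finish event that closes the player and removes the widgets.
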(event OnComponentBeginOverlap(Box)
  (params (OverlappedComponent :type Primitive%20Component%20Object%20Reference) (OtherActor :type Actor%20Object%20Reference) (OtherComp :type Primitive%20Component%20Object%20Reference) (OtherBodyIndex :type Integer) (bFromSweep :type Boolean) (SweepResult :type Hit%20Result%20Structure%20%28by%20ref%29))
  (bind _returnvalue (Game|GetPlayerController 0))
  (Input|EnableInput _returnvalue)
  (Input|SetInputModeGameOnly _returnvalue false)
  (Variables|/Script/Engine.PlayerController|SetbShowMouseCursor _returnvalue false)
  (Utilities|FlowControl|DoOnce false
    (:Completed
      (bind _returnvalue_2 (UserInterface|CreateWidget "/Game/Blueprints/WBP/CutScenes/WBP_Level2StartCutscene.WBP_Level2StartCutscene_C"))
      (bind _output_get (Variables|Default|SetLevel2CutsceneWidget _returnvalue_2))
      (UserInterface|Viewport|AddtoViewport _output_get 0)
      (bind _returnvalue_3 (UserInterface|CreateWidget "/Game/Blueprints/WBP/UI_Overlay/WBP_SkipPrompt.WBP_SkipPrompt_C"))
      (bind _output_get_2 (Variables|Default|SetSkipPromptWidget _returnvalue_3))
      (EventDispatchers|BindEventtoOnSkipCompleted _output_get_2 (delegate Custom|FinishLevel2Cutscene))
      (UserInterface|Viewport|AddtoViewport _output_get_2 10)
      (Variables|Default|SetbCutsceneActive true)
      (Variables|Default|SetbCutsceneFinished false)
      (Media|MediaPlayer|OpenSource (Variables|Default|GetStart%20Cutscene%20Media%20Player) "/Game/Movies/CutsceneLevel2Begining.CutsceneLevel2Begining")
      ;[0.15 0 0.002878 0.5] Change the WBP to the cutscene
      (Utilities|FlowControl|Delay 0.4)
      (Media|MediaPlayer|Play (Variables|Default|GetStart%20Cutscene%20Media%20Player) :!class /Script/MediaAssets.MediaPlayer)
      ;[0.15 0.001527 0 0.5] Change the duration depending on the length of the cutscene
      (Utilities|FlowControl|Delay 74.0)
      (CallFunction|FinishLevel2Cutscene))))

(event Custom|FinishLevel2Cutscene
  (bind _level2cutscenewidget (Variables|Default|GetLevel2CutsceneWidget))
  (bind _skippromptwidget (Variables|Default|GetSkipPromptWidget))
  (if (not (Variables|Default|GetbCutsceneFinished))
    (Variables|Default|SetbCutsceneFinished true)
    (Variables|Default|SetbCutsceneActive false)
    (Media|MediaPlayer|Close (Variables|Default|GetStart%20Cutscene%20Media%20Player) :!class /Script/MediaAssets.MediaPlayer)
    (Utilities|IsValid _level2cutscenewidget
      (:Is%20Valid
        (Widget|RemovefromParent _level2cutscenewidget)
        (Utilities|IsValid _skippromptwidget
          (:Is%20Valid
            (Widget|RemovefromParent _skippromptwidget)))))))

(event Input|EnhancedActionEvents|EnhancedInputActionIA_SkipCutscene
  (params (ActionValue :type Boolean) (ElapsedSeconds :type Float%20%28double-precision%29) (TriggeredSeconds :type Float%20%28double-precision%29) (InputAction :type Input%20Action%20Object%20Reference :default "/Game/Input/Actions/IA_SkipCutscene.IA_SkipCutscene"))
  (bind _skippromptwidget (Variables|Default|GetSkipPromptWidget))
  (bind _skippromptwidget_2 (Variables|Default|GetSkipPromptWidget))
  (:Started
    (Development|PrintString "START SKIP HOLD")
    (if (Variables|Default|GetbCutsceneActive)
      (Utilities|IsValid _skippromptwidget
        (:Is%20Valid
          (Default|StartSkipHold _skippromptwidget)))))
  (:Canceled
    (if (Variables|Default|GetbCutsceneActive) :!label _label
      (Utilities|IsValid _skippromptwidget_2
        (:Is%20Valid
          (Default|StopSkipHold _skippromptwidget_2)))))
  (:Completed
    (goto _label)))

(event Input|EnhancedActionEvents|EnhancedInputActionIA_DialogueAdvance
  (params (ActionValue :type Boolean) (ElapsedSeconds :type Float%20%28double-precision%29) (TriggeredSeconds :type Float%20%28double-precision%29) (InputAction :type Input%20Action%20Object%20Reference :default "/Game/Input/Actions/IA_DialogueAdvance.IA_DialogueAdvance"))
  (bind _skippromptwidget (Variables|Default|GetSkipPromptWidget))
  (bind _skippromptwidget_2 (Variables|Default|GetSkipPromptWidget))
  (:Started
    (Development|PrintString "START SKIP HOLD")
    (if (Variables|Default|GetbCutsceneActive)
      (Utilities|IsValid _skippromptwidget
        (:Is%20Valid
          (Default|StartSkipHold _skippromptwidget)))))
  (:Canceled
    (if (Variables|Default|GetbCutsceneActive) :!label _label
      (Utilities|IsValid _skippromptwidget_2
        (:Is%20Valid
          (Default|StopSkipHold _skippromptwidget_2)))))
  (:Completed
    (goto _label)))

(event EventBeginPlay)

(event Collision|EventActorBeginOverlap
  (params (OtherActor :type Actor%20Object%20Reference)))

(event EventTick
  (params (DeltaSeconds :type Float%20%28single-precision%29)))

(fn ConstructionScript)