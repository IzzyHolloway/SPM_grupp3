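; BP_WaterAI is a particle-bodied water entity with two scripted events: ramming the player's boat and showing itself to the player.
; The hit event shakes the boat's camera, teleports ahead of it, waits, then lerps into its live position via timeline and applies a velocity-change impulse.
; The show event lerps between the current event trigger's start and end positions.
; A timeline that would shift and tilt the boat is never run.
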(event Custom|AI%20Hit%20Event
  (Components|Activation|Activate (Variables|Default|GetParticelBody) false)
  (bind _returnvalue (Actor|GetActorOfClass "/Game/Grupp03_Test/Paula/BP_BoatFunctionality_New.BP_BoatFunctionality_New_C"))
  (Variables|Default|SetBoatFunctionality _returnvalue)
  ;[0.15 0 0 0.5] TODO: Controller Vibration
  (Default|CameraShake (Variables|Default|GetBoatFunctionality))
  (Variables|Default|SetStartLocation (+ (* (Transformation|GetActorForwardVector (Variables|Default|GetBoatFunctionality)) 3e+03) (Transformation|GetActorLocation (Variables|Default|GetBoatFunctionality))))
  (Variables|Default|SetBoatStartLocation (Transformation|GetActorLocation (Variables|Default|GetBoatFunctionality)))
  (Transformation|SetActorLocation (+ (* (Transformation|GetActorForwardVector (Variables|Default|GetBoatFunctionality)) 3e+03) (Transformation|GetActorLocation (Variables|Default|GetBoatFunctionality))) false true)
  (Utilities|FlowControl|Delay 2.0)
  (bind _alpha (Timeline|AIWaterTimeline PlayFromStart)
    (:Update
      (Transformation|SetActorLocation (Math|Vector|Lerp(Vector) (Variables|Default|GetStartLocation) (Transformation|GetActorLocation (Variables|Default|GetBoatFunctionality)) _alpha) false false))
    (:Finished
      (Physics|AddImpulse (Variables|/Script/SPM_grupp3.BoatFunctionality|GetCollisionComponent (Variables|Default|GetBoatFunctionality)) (* (Variables|Default|GetPushPower) (Math|Vector|GetUnitDirection(Vector) (Variables|Default|GetStartLocation) (Transformation|GetActorLocation))) "None" true)
      (Components|Activation|Deactivate (Variables|Default|GetParticelBody)))))

(event Custom|AI%20Show%20To%20Player%20Event
  (bind _current_event_trigger (Variables|Default|GetCurrent%20Event%20Trigger))
  (bind _current_event_trigger_2 (Variables|Default|GetCurrent%20Event%20Trigger))
  (bind _startposition (Variables|/Game/Grupp03_Test/Madde/MaddeBlueprints/BP_WaterAIEventTrigger.BP_WaterAIEventTrigger_C|GetStartPosition _current_event_trigger))
  (Components|Activation|Activate (Variables|Default|GetParticelBody) false)
  (Transformation|SetActorLocation _startposition false true)
  (Development|PrintString (Utilities|String|ToString(Vector) _startposition))
  (bind _alpha (Timeline|AIMoveTimeline Play)
    (:Update
      (Transformation|SetActorLocation (Math|Vector|Lerp(Vector) (Variables|/Game/Grupp03_Test/Madde/MaddeBlueprints/BP_WaterAIEventTrigger.BP_WaterAIEventTrigger_C|GetStartPosition _current_event_trigger_2) (Variables|/Game/Grupp03_Test/Madde/MaddeBlueprints/BP_WaterAIEventTrigger.BP_WaterAIEventTrigger_C|GetEndPosition _current_event_trigger_2) _alpha) false false))
    (:Finished
      (Development|PrintString (Utilities|String|ToString(Vector) (Transformation|GetActorLocation)))
      (Components|Activation|Deactivate (Variables|Default|GetParticelBody)))))

(event EventBeginPlay)

(event Collision|EventActorBeginOverlap
  (params (OtherActor :type Actor%20Object%20Reference)))

(event EventTick
  (params (DeltaSeconds :type Float%20%28single-precision%29)))

(fn ConstructionScript)