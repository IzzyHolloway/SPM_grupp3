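; Shared camera manager for two players that drives a CineCamera according to the active camera zone.
; Each Tick it interpolates the camera toward the players' midpoint plus the zone's offset and toward the zone's rotation.
; SetActiveZone swaps zones and can start a spline transition, which suspends following until progress reaches one.
; During that transition progress advances by the zone's speed, but the spline is always sampled at time zero.
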(event EventBeginPlay
  (bind _asbp_character_speltest_1 (Utilities|Casting|CastToBP_CharacterSpeltest1 (Game|GetPlayerCharacter 0)))
  (Variables|Default|SetPlayer%201 _asbp_character_speltest_1)
  (bind _asbp_character_speltest_1_2 (Utilities|Casting|CastToBP_CharacterSpeltest1 (Game|GetPlayerCharacter 1)))
  (Variables|Default|SetPlayer%202 _asbp_character_speltest_1_2)
  (Game|Player|SetViewTargetwithBlend (Game|GetPlayerController 0) 0 0.5 "VTBlend_Linear" 0.0 false))

(event Collision|EventActorBeginOverlap
  (params (OtherActor :type Actor%20Object%20Reference)))

(event EventTick
  (params (DeltaSeconds :type Float%20%28single-precision%29))
  (bind _cinecamera (Variables|Default|GetCineCamera))
  (if (Variables|Default|GetOnSplineTransition)
    (Variables|Default|SetSplineProgress (CallFunction|SplineProgressCalculation DeltaSeconds))
    (Transformation|SetWorldLocation (Variables|Default|GetCineCamera) (Spline|GetLocationatTime (Variables|/Game/Grupp03_Test/Madde/MaddeBlueprints/BP_CameraZone.BP_CameraZone_C|GetTransitionSpline (Variables|Default|GetActiveZone)) 0.0 "Local" false) false false)
    (if (>= (Variables|Default|GetSplineProgress) 1.0)
      (Variables|Default|SetOnSplineTransition false))
    (else
      (Transformation|SetWorldLocation _cinecamera (Math|Interpolation|VInterpTo (Variables|/Script/Engine.SceneComponent|GetRelativeLocation _cinecamera) (CallFunction|SetTargetLocation) DeltaSeconds (Variables|/Game/Grupp03_Test/Madde/MaddeBlueprints/BP_CameraZone.BP_CameraZone_C|GetTransitionSpeed (Variables|Default|GetActiveZone))) false false)
      (Transformation|SetRelativeRotation (Variables|Default|GetCineCamera) (Math|Interpolation|RInterpTo (Variables|/Script/Engine.SceneComponent|GetRelativeRotation (Variables|Default|GetCineCamera)) (Variables|/Game/Grupp03_Test/Madde/MaddeBlueprints/BP_CameraZone.BP_CameraZone_C|GetCameraRotation (Variables|Default|GetActiveZone)) DeltaSeconds 0.0) false false))))

(fn ConstructionScript)

(fn SetActiveZone
  (params (NewZone :type BP%20Camera%20Zone%20Object%20Reference))
  (bind _output_get (Variables|Default|SetActiveZone NewZone))
  (Variables|/Game/Grupp03_Test/Madde/MaddeBlueprints/BP_CameraZone.BP_CameraZone_C|GetHasSplineTransition _output_get
    (:then
      (Variables|Default|SetOnSplineTransition true)
      (Variables|Default|SetSplineProgress 0.0))
    (:else)))

(fn SetTargetLocation
  (return (+ (Variables|/Game/Grupp03_Test/Madde/MaddeBlueprints/BP_CameraZone.BP_CameraZone_C|GetCameraOffset (Variables|Default|GetActiveZone)) (/ (+ (Transformation|GetActorLocation (Variables|Default|GetPlayer%201)) (Transformation|GetActorLocation (Variables|Default|GetPlayer%202))) 2.0))))

(fn SplineProgressCalculation
  (params (InputPin :type Float%20%28single-precision%29))
  (return (+ (Variables|Default|GetSplineProgress) (* InputPin (Variables|/Game/Grupp03_Test/Madde/MaddeBlueprints/BP_CameraZone.BP_CameraZone_C|GetTransitionSpeed (Variables|Default|GetActiveZone))))))