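; An overlap trigger actor that starts AI gameplay events when something enters its box.
; On overlap begin it finds the BP_AIGameplay actor, registers itself as that actor's current event trigger and calls either the deck or stone AI event, chosen by an IsBridgeIsland flag.
; It tracks box occupancy in IsInBox and prints a debug string for each branch, without filtering the overlapping actor.
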(event OnComponentBeginOverlap(Box)
  (params (OverlappedComponent :type Primitive%20Component%20Object%20Reference) (OtherActor :type Actor%20Object%20Reference) (OtherComp :type Primitive%20Component%20Object%20Reference) (OtherBodyIndex :type Integer) (bFromSweep :type Boolean) (SweepResult :type Hit%20Result%20Structure%20%28by%20ref%29))
  (Variables|Default|SetIsInBox true)
  (bind _returnvalue (Actor|GetActorOfClass "/Game/Grupp03_Test/Madde/MaddeBlueprints/BP_AIGameplay.BP_AIGameplay_C"))
  (Variables|/Game/Grupp03_Test/Madde/MaddeBlueprints/BP_AIGameplay.BP_AIGameplay_C|SetCurrent%20Event%20Trigger _returnvalue self)
  (if (Variables|Default|GetIsBridgeIsland)
    (Development|PrintString "We have triggered bridge AI!")
    (Default|AIDeckEvent _returnvalue)
    (else
      (Development|PrintString "We have triggered stone AI!")
      (Default|AIStoneEvent _returnvalue))))

(event OnComponentEndOverlap(Box)
  (params (OverlappedComponent :type Primitive%20Component%20Object%20Reference) (OtherActor :type Actor%20Object%20Reference) (OtherComp :type Primitive%20Component%20Object%20Reference) (OtherBodyIndex :type Integer))
  (Variables|Default|SetIsInBox false))

(event EventBeginPlay)

(event Collision|EventActorBeginOverlap
  (params (OtherActor :type Actor%20Object%20Reference)))

(event EventTick
  (params (DeltaSeconds :type Float%20%28single-precision%29)))

(fn ConstructionScript)