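; Cutscene manager actor that briefly takes over the first player's view for a cutscene, triggered by pressing the 1 key with a debug print.
; Cutscene1 moves the actor to a stored location and rotation and makes itself the view target.
; After a short delay, it hands the view to the BP_CameraDirector found in the level.
; A swoosh sound node exists but is never run.
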(event Custom|Cut%20scene%201
  (bind _returnvalue (Game|GetPlayerController 0))
  (Transformation|SetActorLocation (Variables|Default|GetCutscene1Location) false false)
  (Transformation|SetActorRotation (Variables|Default|GetCutscene1Rotation))
  (Game|Player|SetViewTargetwithBlend _returnvalue self 0.0 "VTBlend_Linear" 0.0 false)
  (Utilities|FlowControl|Delay 2.0)
  (bind _returnvalue_2 (Actor|GetActorOfClass "/Game/Grupp03_Test/Madde/MaddeBlueprints/BP_CameraDirector.BP_CameraDirector_C"))
  (Game|Player|SetViewTargetwithBlend _returnvalue _returnvalue_2 0.0 "VTBlend_Linear" 0.0 false))

(event EventBeginPlay)

(event Collision|EventActorBeginOverlap
  (params (OtherActor :type Actor%20Object%20Reference)))

(event EventTick
  (params (DeltaSeconds :type Float%20%28single-precision%29)))

(event Input|KeyboardEvents|1
  (params (Key :type Key%20Structure))
  (:Pressed
    (Development|PrintString "We haved pressed 1")
    (CallFunction|CutScene1)))

(fn ConstructionScript)