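; BP_DoorInteractable is a door that teleports the player between paired inside and outside positions.
; OnDoorInteract plays a door sound and shows a WBP_BlackFade, which it fades back and removes after a short delay.
; The BP_CameraDirector's active zone decides the direction and is then switched to the destination zone.
; Entering enables the fixed camera, while exiting disables it and snaps the director to the outside position plus zone offset.
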(event EventBeginPlay)

(event Collision|EventActorBeginOverlap
  (params (OtherActor :type Actor%20Object%20Reference)))

(event EventTick
  (params (DeltaSeconds :type Float%20%28single-precision%29)))

(event EventOnDoorInteract
  (bind _returnvalue (Game|GetPlayerCharacter 0))
  (bind _returnvalue_2 (UserInterface|CreateWidget "/Game/Grupp03_Test/Madde/Widget/WBP_BlackFade.WBP_BlackFade_C"))
  (UserInterface|Viewport|AddtoViewport _returnvalue_2 0)
  (Audio|PlaySound2D "/Game/Grupp03_Test/Zoey/Audio/SC_Door.SC_Door" 1.0 1.0 0.0 0 0)
  (Default|FadeScreen _returnvalue_2 true)
  (bind _returnvalue_3 (Actor|GetActorOfClass "/Game/Grupp03_Test/Madde/MaddeBlueprints/BP_CameraDirector.BP_CameraDirector_C"))
  (if (Variables|/Game/Grupp03_Test/Madde/MaddeBlueprints/BP_CameraZone.BP_CameraZone_C|GetIsInside (Variables|/Game/Grupp03_Test/Madde/MaddeBlueprints/BP_CameraDirector.BP_CameraDirector_C|GetActiveZone _returnvalue_3))
    (Transformation|SetActorLocation _returnvalue (Variables|Default|GetOutsidePosition) false true)
    (bind _returnvalue_4 (Actor|GetActorOfClass "/Game/Grupp03_Test/Madde/MaddeBlueprints/BP_CameraDirector.BP_CameraDirector_C"))
    (Variables|/Game/Grupp03_Test/Madde/MaddeBlueprints/BP_CameraDirector.BP_CameraDirector_C|SetbFixedCamera _returnvalue_4 false)
    (bind _returnvalue_5 (Actor|GetActorOfClass "/Game/Grupp03_Test/Madde/MaddeBlueprints/BP_CameraDirector.BP_CameraDirector_C"))
    (bind _output_get (Variables|/Game/Grupp03_Test/Madde/MaddeBlueprints/BP_CameraDirector.BP_CameraDirector_C|SetActiveZone _returnvalue_5 (Variables|Default|GetOutsideZone)))
    (Transformation|SetActorLocation _returnvalue_5 (+ (Variables|/Game/Grupp03_Test/Madde/MaddeBlueprints/BP_CameraZone.BP_CameraZone_C|GetCameraOffset _output_get) (Variables|Default|GetOutsidePosition)) false true)
    (else
      (Transformation|SetActorLocation _returnvalue (Variables|Default|GetInsidePosition) false true)
      (bind _returnvalue_6 (Actor|GetActorOfClass "/Game/Grupp03_Test/Madde/MaddeBlueprints/BP_CameraDirector.BP_CameraDirector_C"))
      (Variables|/Game/Grupp03_Test/Madde/MaddeBlueprints/BP_CameraDirector.BP_CameraDirector_C|SetbFixedCamera _returnvalue_6 true)
      (bind _returnvalue_7 (Actor|GetActorOfClass "/Game/Grupp03_Test/Madde/MaddeBlueprints/BP_CameraDirector.BP_CameraDirector_C"))
      (Variables|/Game/Grupp03_Test/Madde/MaddeBlueprints/BP_CameraDirector.BP_CameraDirector_C|SetActiveZone _returnvalue_7 (Variables|Default|GetInsideZone))))
  (Utilities|FlowControl|Delay 1.0)
  (Default|FadeScreen _returnvalue_2 false)
  (Widget|RemovefromParent _returnvalue_2))

(fn ConstructionScript)