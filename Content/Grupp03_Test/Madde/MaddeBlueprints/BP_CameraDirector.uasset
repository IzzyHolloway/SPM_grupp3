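; Camera director actor that acts as the player's view, driven by the active BP_CameraZone, and stages the game's intro and cutscenes.
; BeginPlay locks movement during a black fade, shows intro narration, then takes the view and finds the player's zone if possessed.
; Tick either snaps to the zone's related door or, outdoors, interpolates toward player-relative offset and zone rotation.
; Island and home cutscene events suspend tracking at preset transforms until StopCutscene; temporary keys trigger two.
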(event Custom|PanBackCameraRotation
  ;[0.15 0.15 0.15 0.5] Place camera back to its original rotation
  (Transformation|SetActorRotation (Math|Rotator|Lerp(Rotator) (Transformation|GetActorRotation self) (Variables|/Game/Grupp03_Test/Madde/MaddeBlueprints/BP_CameraZone.BP_CameraZone_C|GetCameraRotation (Variables|Default|GetActiveZone)) 0.0)))

(event Custom|Cutscene%20Home
  ;[0.15 0.15 0.15 0.5] Cutscene after crafting the lantern
  (Variables|Default|SetIsInCutScene true)
  (Transformation|SetActorLocation (Variables|Default|GetCutsceneLocationHome) false false)
  (Transformation|SetActorRotation (Variables|Default|GetCutsceneRotationHome))
  (Utilities|FlowControl|Delay 2.0))

(event Custom|CutScene%201
  ;[0.15 0.15 0.15 0.5] Cutscene after completing puzzle island 1
  (Variables|Default|SetIsInCutScene true)
  (Transformation|SetActorLocation (Variables|Default|GetCutsceneLocationIsland1) false false)
  (Transformation|SetActorRotation (Variables|Default|GetCutsceneRotationIsland1))
  (Utilities|FlowControl|Delay 1.0)
  (Utilities|FlowControl|Delay 2.0))

(event Custom|Stop%20Cutscene
  (Variables|Default|SetIsInCutScene false))

(event Custom|Cutscene%202
  ;[0.15 0.15 0.15 0.5] Cutscene after completing puzzle island 2
  (Variables|Default|SetIsInCutScene true)
  (Transformation|SetActorLocation (Variables|Default|GetCutsceneLocationIsland2) false false)
  (Transformation|SetActorRotation (Variables|Default|GetCutsceneRotationIsland2))
  (Utilities|FlowControl|Delay 2.0))

(event EventBeginPlay
  ;[0.15 0.15 0.15 0.5] "Cutscene" when you start the game
  (bind _returnvalue (Actor|GetActorOfClass "/Game/Grupp03_Test/Speltest1/BP_CharacterSpeltest1.BP_CharacterSpeltest1_C"))
  (Class|CharacterAimi|SetMovementLocked _returnvalue true)
  (bind _returnvalue_2 (UserInterface|CreateWidget "/Game/Grupp03_Test/Madde/Widget/WBP_BlackFade.WBP_BlackFade_C"))
  (UserInterface|Viewport|AddtoViewport _returnvalue_2 0)
  (Default|FadeScreen _returnvalue_2 true)
  (Utilities|FlowControl|Delay 2.0)
  (Default|FadeScreen _returnvalue_2 false)
  (Widget|RemovefromParent _returnvalue_2)
  (bind _returnvalue_3 (UserInterface|CreateWidget "/Game/Blueprints/WBP/WBP_IntroScreenNarration.WBP_IntroScreenNarration_C"))
  (UserInterface|Viewport|AddtoViewport _returnvalue_3 0)
  (Class|CharacterAimi|SetMovementLocked _returnvalue false)
  (Input|EnableInput self (Game|GetPlayerController 0))
  (bind _returnvalue_4 (Actor|GetActorOfClass "/Game/Grupp03_Test/Speltest1/BP_CharacterSpeltest1.BP_CharacterSpeltest1_C"))
  (if (Variables|/Game/Grupp03_Test/Speltest1/BP_CharacterSpeltest1.BP_CharacterSpeltest1_C|GetPossessed _returnvalue_4)
    (Game|Player|SetViewTargetwithBlend (Game|GetPlayerController 0) self 0.0 "VTBlend_Linear" 0.0 false)
    (Actor|GetAllActorsOfClass "/Game/Grupp03_Test/Madde/MaddeBlueprints/BP_CameraZone.BP_CameraZone_C")
    (bind _array_element (Utilities|Array|ForEachLoopwithBreak 0 :!label _label)
      (:LoopBody
        (if (not (Utilities|Array|IsEmpty (Collision|GetOverlappingActors _array_element "/Game/Grupp03_Test/Speltest1/BP_CharacterSpeltest1.BP_CharacterSpeltest1_C" :!class /Script/Engine.Actor)))
          (Variables|Default|SetActiveZone _array_element)
          (goto _label Break))))))

(event Collision|EventActorBeginOverlap
  (params (OtherActor :type Actor%20Object%20Reference)))

(event EventTick
  (params (DeltaSeconds :type Float%20%28single-precision%29))
  (bind _activezone (Variables|Default|GetActiveZone))
  (bind _activezone_2 (Variables|Default|GetActiveZone))
  (bind _cinecamera (Variables|Default|GetCineCamera))
  (bind _relateddoor (Variables|/Game/Grupp03_Test/Madde/MaddeBlueprints/BP_CameraZone.BP_CameraZone_C|GetRelatedDoor _activezone_2))
  ;[0.15 0.15 0.15 0.5] Handles the camera when the player moves around in the world
  (if (not (Variables|Default|GetIsInCutScene))
    (if (Utilities|IsValid (Variables|Default|GetActiveZone))
      (if (Variables|Default|GetbFixedCamera)
        (if (Utilities|IsValid _relateddoor)
          (Transformation|SetActorLocation (+ (Variables|/Game/Grupp03_Test/Madde/MaddeBlueprints/BP_DoorInteractable.BP_DoorInteractable_C|GetInsidePosition _relateddoor) (Variables|/Game/Grupp03_Test/Madde/MaddeBlueprints/BP_CameraZone.BP_CameraZone_C|GetCameraOffset _activezone)) false true)
          (Transformation|SetActorRelativeRotation self (Variables|/Game/Grupp03_Test/Madde/MaddeBlueprints/BP_CameraZone.BP_CameraZone_C|GetCameraRotation _activezone)))
        (elif (not (Variables|/Game/Grupp03_Test/Madde/MaddeBlueprints/BP_CameraZone.BP_CameraZone_C|GetIsInside (Variables|Default|GetActiveZone)))
          (bind _returnvalue (CallFunction|FindCameraLocation (Transformation|GetActorLocation (Game|GetPlayerCharacter 0))))
          (Transformation|SetActorLocation _returnvalue false false)
          (bind _returnvalue_2 (CallFunction|FindCameraRotation (Utilities|Time|GetWorldDeltaSeconds)))
          (Transformation|SetActorRotation _returnvalue_2)
          (Transformation|SetRelativeRotation _cinecamera (Math|Interpolation|RInterpTo (Variables|/Script/Engine.SceneComponent|GetRelativeRotation _cinecamera) (Variables|Default|GetPlayerRotationOffset) (Utilities|Time|GetWorldDeltaSeconds) 2.0) false false))))))

(event Input|KeyboardEvents|DebugKeyR
  (params (Key :type Key%20Structure :default "None") (ActionValue :type Input%20Action%20Value%20Structure))
  ;[0.15 0.15 0.15 0.5] Temporary test keys
  (:Pressed
    (CallFunction|CutsceneHome)))

(event Input|KeyboardEvents|1
  (params (Key :type Key%20Structure :default "None"))
  ;[0.15 0.15 0.15 0.5] Temporary test keys
  (:Pressed
    (CallFunction|Cutscene2)))

(fn ConstructionScript)

(fn FindCameraLocation
  (params (A :type Vector))
  (if (Utilities|IsValid (Variables|Default|GetActiveZone))
    (return (Math|Interpolation|VInterpTo (Transformation|GetActorLocation self) (+ (+ A "") (Variables|/Game/Grupp03_Test/Madde/MaddeBlueprints/BP_CameraZone.BP_CameraZone_C|GetCameraOffset (Variables|Default|GetActiveZone))) (Utilities|Time|GetWorldDeltaSeconds) 2.0))
    (else
      (return "0, 0, 0"))))

(fn FindCameraRotation
  (params (DeltaTime :type Float%20%28single-precision%29))
  (if (Utilities|IsValid (Variables|Default|GetActiveZone))
    (return (Math|Interpolation|RInterpTo (Transformation|GetActorRotation self) (Variables|/Game/Grupp03_Test/Madde/MaddeBlueprints/BP_CameraZone.BP_CameraZone_C|GetCameraRotation (Variables|Default|GetActiveZone)) DeltaTime 2.0))))

(fn SplineProgressCalculation
  (params (Input :type Float%20%28double-precision%29))
  (return (+ (Variables|Default|GetSplineProgress) (* Input (Variables|/Game/Grupp03_Test/Madde/MaddeBlueprints/BP_CameraZone.BP_CameraZone_C|GetTransitionSpeed (Variables|Default|GetActiveZone))))))