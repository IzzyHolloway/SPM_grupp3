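; BP_StonePuzzle is a puzzle controller that repeatedly shows the code sequence by lowering stones.
; From BeginPlay it steps through CorrectCode as one-based indices into StoneArray, calling MoveStoneDown with timed delays, then pauses and restarts until PuzzleFinished.
; PuzzleComplete, not called within this graph, completes every stone, sets PuzzleFinished to stop the loop and destroys the blocking volumes.
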(event Custom|Play%20Puzzle
  (Variables|Default|SetCurrentIndex 0)
  (CallFunction|PlayNextStone))

(event Custom|Play%20Next%20Stone
  (bind _correctcode (Variables|Default|GetCorrectCode))
  (if (not (Variables|Default|GetPuzzle%20Finished))
    (if (Utilities|Array|IsValidIndex _correctcode (Variables|Default|GetCurrentIndex))
      (Default|MoveStoneDown (Utilities|Array|Get(acopy) (Variables|Default|GetStoneArray) (- (Utilities|Array|Get(acopy) _correctcode (Variables|Default|GetCurrentIndex)) 1)))
      (Utilities|FlowControl|Delay 5.0)
      (Variables|Default|SetCurrentIndex (+ (Variables|Default|GetCurrentIndex) 1))
      (CallFunction|PlayNextStone)
      (else
        (Utilities|FlowControl|Delay 3.0)
        (CallFunction|PlayPuzzle)))))

(event Custom|Puzzle%20Complete
  (for _array_element (Variables|Default|GetStoneArray)
    (Default|CompletePuzzle _array_element)
    (Variables|Default|SetPuzzle%20Finished true)
    (for _array_element_2 (Variables|Default|GetBlockingVolume1)
      (Utilities|IsValid _array_element_2
        (:Is%20Valid
          (Actor|DestroyActor _array_element_2))))))

(event EventBeginPlay
  (if true
    (CallFunction|PlayPuzzle)))

(event Collision|EventActorBeginOverlap
  (params (OtherActor :type Actor%20Object%20Reference)))

(event EventTick
  (params (DeltaSeconds :type Float%20%28single-precision%29)))

(fn ConstructionScript)