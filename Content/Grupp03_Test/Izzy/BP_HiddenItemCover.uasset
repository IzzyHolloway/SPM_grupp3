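; BP_HiddenItemCover is an interactable cover that hides a linked pickup by disabling that pickup's collision on BeginPlay.
; A sphere overlap enables input and shows a prompt widget; leaving disables input and hides it.
; On Interact, the Item component rises with a sound and the pickup's collision turns on.
; After a delay it lowers, then input and widget switch off, while pickup collision stays enabled.
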(event OnComponentBeginOverlap(Sphere)
  (params (OverlappedComponent :type Primitive%20Component%20Object%20Reference) (OtherActor :type Actor%20Object%20Reference) (OtherComp :type Primitive%20Component%20Object%20Reference) (OtherBodyIndex :type Integer) (bFromSweep :type Boolean) (SweepResult :type Hit%20Result%20Structure%20%28by%20ref%29))
  ;[0.15 0.15 0.15 0.5] Toggles input based on proximity and hides the pickup's collision at start. On Interact: Reveals the pickup, enables its collision so it can be gathered, and auto-closes after 1.5 seconds. + UI visibility
  (Input|EnableInput (Game|GetPlayerController 0))
  (Rendering|SetVisibility (Variables|Default|GetWidget) true false))

(event OnComponentEndOverlap(Sphere)
  (params (OverlappedComponent :type Primitive%20Component%20Object%20Reference) (OtherActor :type Actor%20Object%20Reference) (OtherComp :type Primitive%20Component%20Object%20Reference) (OtherBodyIndex :type Integer))
  ;[0.15 0.15 0.15 0.5] Toggles input based on proximity and hides the pickup's collision at start. On Interact: Reveals the pickup, enables its collision so it can be gathered, and auto-closes after 1.5 seconds. + UI visibility
  (Input|DisableInput (Game|GetPlayerController 0))
  (Rendering|SetVisibility (Variables|Default|GetWidget) false false))

(event Input|EnhancedActionEvents|EnhancedInputActionIA_Interact
  (params (ActionValue :type Boolean) (ElapsedSeconds :type Float%20%28double-precision%29) (TriggeredSeconds :type Float%20%28double-precision%29) (InputAction :type Input%20Action%20Object%20Reference :default "/Game/Input/Actions/IA_Interact.IA_Interact"))
  ;[0.15 0.15 0.15 0.5] Toggles input based on proximity and hides the pickup's collision at start. On Interact: Reveals the pickup, enables its collision so it can be gathered, and auto-closes after 1.5 seconds. + UI visibility
  (:Started
    (Audio|PlaySound2D "/Game/Grupp03_Test/Zoey/Audio/LiftStoneUp.LiftStoneUp" 1.0 1.0 0.0 0 0)
    (Components|MoveComponentTo (Variables|Default|GetItem) "0.000000,0.000000,200.000000" "0, 0, 0" false false 0.7 false)
    (Utilities|IsValid (Variables|Default|GetMyHiddenPickup)
      (:Is%20Valid
        (Collision|SetActorEnableCollision (Variables|Default|GetMyHiddenPickup) true))
      (:Is%20Not%20Valid
        _))
    (Utilities|FlowControl|Delay 1.5)
    (Audio|PlaySound2D "/Game/Grupp03_Test/Zoey/Audio/liftStoneDown.liftStoneDown" 1.0 1.0 0.0 0 0)
    (Components|MoveComponentTo (Variables|Default|GetItem) "0, 0, 0" "0, 0, 0" false false 2.0 false)
    (Input|DisableInput (Game|GetPlayerController 0))
    (Rendering|SetVisibility (Variables|Default|GetWidget) false false)))

(event EventBeginPlay
  ;[0.15 0.15 0.15 0.5] Toggles input based on proximity and hides the pickup's collision at start. On Interact: Reveals the pickup, enables its collision so it can be gathered, and auto-closes after 1.5 seconds. + UI visibility
  (Utilities|IsValid (Variables|Default|GetMyHiddenPickup)
    (:Is%20Valid
      (Collision|SetActorEnableCollision (Variables|Default|GetMyHiddenPickup) false))))

(fn ConstructionScript)