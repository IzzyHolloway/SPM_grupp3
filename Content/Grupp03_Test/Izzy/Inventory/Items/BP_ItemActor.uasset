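; BP_ItemActor is a pickup item that the player collects into their inventory.
; Interacting adds the ID and quantity from BPCItemData to the player character's Inventory, then plays a pickup sound and destroys the actor on success.
; EndPlay also plays that sound for any end reason, as the Destroyed-only check is disconnected.
; LookAtActor returns the item's name from the DT_ItemData_NEW data table.
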(event EventEndPlay
  (params (EndPlayReason :type EEndPlayReason%20Enum :default "Destroyed"))
  (Audio|PlaySound2D (Variables|Default|GetS_PickupSound) 1.0 1.0 0.0 0 0))

(event EventInteractwith
  (params (Interactor :type Actor%20Object%20Reference))
  (bind _bpc_itemdata (Variables|Default|GetBPC_ItemData))
  (bind _asbp_character_speltest_1 (Utilities|Casting|CastToBP_CharacterSpeltest1 (Game|GetPlayerCharacter 0)))
  (bind _returnvalue (Class|InventoryComponent|AddItemtoInventory (Variables|/Game/Grupp03_Test/Speltest1/BP_CharacterSpeltest1.BP_CharacterSpeltest1_C|GetInventory _asbp_character_speltest_1) (Variables|/Game/Grupp03_Test/Izzy/Inventory/InventoryAndCrafting/BPC_ItemData.BPC_ItemData_C|GetItemID _bpc_itemdata) (Variables|/Game/Grupp03_Test/Izzy/Inventory/InventoryAndCrafting/BPC_ItemData.BPC_ItemData_C|GetItemQuantity _bpc_itemdata)))
  (if _returnvalue
    (Development|PrintString "Hello")
    (Audio|PlaySound2D (Variables|Default|GetS_PickupSound) 1.0 1.0 0.0 0 0)
    (Actor|DestroyActor)))

(fn ConstructionScript)

(fn LookatActor
  (bind _returnvalue (Utilities|GetDataTableRow "/Game/Grupp03_Test/Izzy/Inventory/InventoryAndCrafting/DT_ItemData_NEW.DT_ItemData_NEW" (Variables|/Game/Grupp03_Test/Izzy/Inventory/InventoryAndCrafting/BPC_ItemData.BPC_ItemData_C|GetItemID (Variables|Default|GetBPC_ItemData)))
    (:then
      (return (.ItemName (Utilities|Struct|BreakItemDetail _returnvalue))))))