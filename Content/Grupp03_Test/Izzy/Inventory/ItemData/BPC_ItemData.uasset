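; BPC_ItemData is an item component that lets its owning actor be picked up into the player's inventory.
; On interaction, it finds BPC_Inventory on the first player character and passes it the ItemData row name, destroying the owner if the add succeeds.
; A DoOnce with no reset allows only one attempt, even if the add fails.
; LookAtActor returns an empty string.
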(event EventBeginPlay)

(event EventTick
  (params (DeltaSeconds :type Float%20%28single-precision%29)))

(event EventInteractwith
  (bind _returnvalue (Game|GetPlayerCharacter 0))
  (bind _returnvalue_2 (Actor|GetComponentbyClass _returnvalue "/Game/Grupp03_Test/Izzy/Inventory/BPC_Inventory.BPC_Inventory_C"))
  (Utilities|FlowControl|DoOnce false
    (:Completed
      (Utilities|IsValid _returnvalue_2
        (:Is%20Valid
          (bind _isinventory (Default|AddtoInventory _returnvalue_2 (.RowName (Utilities|Struct|BreakDataTableRowHandle (Variables|Default|GetItemData)))))
          (if _isinventory
            (Actor|DestroyActor (Components|GetOwner))))))))

(fn LookatActor
  (return ""))