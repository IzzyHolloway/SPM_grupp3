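; Inventory component that holds a fixed-size array of slots, each storing one item ID, with "None" marking an empty slot.
; Adding fills the first empty slot or reports full; transfers swap slots between inventories, and ReturnItems moves another inventory's items into this one.
; Changes broadcast through OnInventoryUpdated, and item details come from DT_ItemData.
; IA_Inventory toggles the WB_PlayerInventory widget unless locked, and key 1 prints slots.
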(event Custom|UpdateInventory
  (Default|CallOnInventoryUpdated))

(event Input|EnhancedActionEvents|EnhancedInputActionIA_Inventory
  (params (ActionValue :type Boolean) (ElapsedSeconds :type Float%20%28double-precision%29) (TriggeredSeconds :type Float%20%28double-precision%29) (InputAction :type Input%20Action%20Object%20Reference :default "/Game/Input/Actions/IA_Inventory.IA_Inventory"))
  (:Started
    (if (not (Variables|Default|GetIsLocked))
      (CallFunction|ToggleInventory))))

(event EventBeginPlay
  (Utilities|Array|Resize (Variables|Default|GetInventorySlots) (Variables|Default|GetInventorySize)))

(event EventTick
  (params (DeltaSeconds :type Float%20%28single-precision%29)))

(event Input|KeyboardEvents|1
  (params (Key :type Key%20Structure :default "None"))
  (:Pressed
    (CallFunction|PrintInventory)))

(fn PrintInventory
  (for (_array_element _array_index) (Variables|Default|GetInventorySlots)
    (Development|PrintString (Utilities|String|Append (Utilities|String|ToString(Integer) _array_index) ":" (Utilities|String|ToString(Name) (Utilities|Struct|BreakS_InventorySlot _array_element))))))

(fn AddtoInventory
  (params (ItemID :type Name))
  (bind (_index _found) (CallFunction|AnySlotsAvailable))
  (if _found
    (CallFunction|CreateNewStack _index ItemID)
    (Utilities|Array|SetArrayElem (Variables|Default|GetInventorySlots) _index (Utilities|Struct|MakeS_InventorySlot ItemID))
    (else
      (LocalVariables|SetLocal_IsInventoryFull true)))
  (CallFunction|UpdateInventory)
  (return (LocalVariables|GetLocal_IsInventoryFull)))

(fn FindMatchingSlot
  (params (ItemID :type Name))
  (for (_array_element _array_index) (Variables|Default|GetInventorySlots)
    (if (== (Utilities|Struct|BreakS_InventorySlot _array_element) ItemID)
      (return _array_index true)))
  (return -1 false))

(fn GetItemDetails
  (params (ItemID :type Name))
  (bind _returnvalue (Utilities|GetDataTableRow "/Game/Grupp03_Test/Izzy/Inventory/ItemData/DT_ItemData.DT_ItemData" ItemID)
    (:then
      (return _returnvalue))))

(fn AddItemtoStack
  (params (Index :type Integer))
  (Utilities|Array|SetArrayElem (Variables|Default|GetInventorySlots) Index (Utilities|Struct|MakeS_InventorySlot (Utilities|Struct|BreakS_InventorySlot (Utilities|Array|Get(acopy) (Variables|Default|GetInventorySlots) Index)))))

(fn AnySlotsAvailable
  (for (_array_element _array_index) (Variables|Default|GetInventorySlots)
    (if (== (Utilities|Struct|BreakS_InventorySlot _array_element) "")
      (return _array_index true)))
  (return -1 false))

(fn CreateNewStack
  (params (Index :type Integer) (ItemID :type Name))
  (Utilities|Array|SetArrayElem (Variables|Default|GetInventorySlots) Index (Utilities|Struct|MakeS_InventorySlot ItemID)))

(fn ToggleInventory
  (bind _playerinventorywidget (Variables|Default|GetPlayerInventoryWidget)
    (:then
      (Widget|RemovefromParent _playerinventorywidget)
      (Variables|Default|SetPlayerInventoryWidget 0))
    (:else
      (bind _returnvalue (UserInterface|CreateWidget "/Game/Grupp03_Test/Izzy/Inventory/UI/InventoryUI/WB_PlayerInventory.WB_PlayerInventory_C"))
      (bind _output_get (Variables|Default|SetPlayerInventoryWidget _returnvalue))
      (UserInterface|Viewport|AddtoViewport _output_get 0))))

(fn TransferSlots
  (params (Index :type Integer) (SourceInventory :type BPC%20Inventory%20Object%20Reference) (SourceIndex :type Integer))
  (LocalVariables|SetLocalItem (Utilities|Array|Get(acopy) (Variables|Default|GetInventorySlots) Index))
  (LocalVariables|SetLocalSourceItem (Utilities|Array|Get(acopy) (Variables|BPC_Inventory_C|GetInventorySlots SourceInventory) SourceIndex))
  (Utilities|FlowControl|Sequence
    (:then_0
      (CallFunction|CreateNewStack Index (.itemid (LocalVariables|GetLocalSourceItem))) ; Target Inventory
      (CallFunction|CreateNewStack SourceInventory SourceIndex (.itemid (LocalVariables|GetLocalItem))) ; Source Inventory
    )
    (:then_1
      (CallFunction|UpdateInventory)
      (CallFunction|UpdateInventory SourceInventory))))

(fn ReturnItems
  (params (SourceInventory :type BPC%20Inventory%20Object%20Reference))
  (bind _inventoryslots (Variables|BPC_Inventory_C|GetInventorySlots SourceInventory))
  (for _array_element (Variables|BPC_Inventory_C|GetInventorySlots SourceInventory)
    (if (!= (Utilities|Struct|BreakS_InventorySlot _array_element) "")
      (CallFunction|AddtoInventory (Utilities|Struct|BreakS_InventorySlot _array_element))))
  (Utilities|Array|Clear _inventoryslots)
  (Utilities|Array|Resize _inventoryslots (Variables|BPC_Inventory_C|GetInventorySize SourceInventory))
  (CallFunction|UpdateInventory SourceInventory))

(fn GetItemIDs
  (for _array_element (Variables|Default|GetInventorySlots)
    (Utilities|Array|Add (LocalVariables|GetLocalItemIDs) (Utilities|Struct|BreakS_InventorySlot _array_element)))
  (return (LocalVariables|GetLocalItemIDs)))

(fn RemovefromStack
  (params (Index :type Integer))
  (Utilities|Array|SetArrayElem (Variables|Default|GetInventorySlots) Index (Utilities|Struct|MakeS_InventorySlot "None"))
  (CallFunction|UpdateInventory))