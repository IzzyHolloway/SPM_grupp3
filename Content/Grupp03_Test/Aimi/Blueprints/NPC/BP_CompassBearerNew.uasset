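; Compass bearer NPC that stays hidden and non-colliding until ShowCompassBearer reveals it on the player's island.
; The reveal teleports it to the lever or motor island transform, whichever is closer to the player, and enables ForceTalkTrigger.
; The player's first overlap disables that trigger and starts AutoDialogueData through BP_DialogueManager.
; A tagged spawn-point search goes uncalled here, and progression-flag placement is disconnected.
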(event OnComponentBeginOverlap(ForceTalkTrigger)
  (params (OverlappedComponent :type Primitive%20Component%20Object%20Reference) (OtherActor :type Actor%20Object%20Reference) (OtherComp :type Primitive%20Component%20Object%20Reference) (OtherBodyIndex :type Integer) (bFromSweep :type Boolean) (SweepResult :type Hit%20Result%20Structure%20%28by%20ref%29))
  (Utilities|Casting|CastToCharacterAimi OtherActor)
  (if (not (Variables|Default|GetbHasTriggeredDialogue))
    (Variables|Default|SetbHasTriggeredDialogue true)
    (Collision|SetCollisionEnabled (Variables|Default|GetForceTalkTrigger) "NoCollision")
    (bind _returnvalue (Actor|GetActorOfClass "/Game/Grupp03_Test/Aimi/Blueprints/Managers/BP_DialogueManager.BP_DialogueManager_C"))
    (Class|DialogueManager|StartDialoguefromDataAsset _returnvalue (Variables|Default|GetAutoDialogueData))))

(event Custom|ShowCompassBearer
  (CallFunction|MoveCompassBearertoPlayerIsland)
  (Rendering|SetActorHiddenInGame false)
  (Collision|SetActorEnableCollision true)
  (Collision|SetCollisionEnabled (Variables|Default|GetForceTalkTrigger) "QueryOnly"))

(event Custom|MoveCompassBearerToPlayerIsland
  (bind _returnvalue (Game|GetPlayerCharacter 0))
  (bind _returnvalue_2 (Transformation|GetActorLocation _returnvalue))
  (if (<= (Math|Vector|Distance(Vector) _returnvalue_2 (.location (Variables|Default|GetLeverIslandSpawnTransform))) (Math|Vector|Distance(Vector) _returnvalue_2 (.location (Variables|Default|GetMotorIslandSpawnTransform))))
    (Transformation|SetActorTransform (Variables|Default|GetLeverIslandSpawnTransform))
    (else
      (Transformation|SetActorTransform (Variables|Default|GetMotorIslandSpawnTransform)))))

(event EventBeginPlay
  (Rendering|SetActorHiddenInGame true)
  (Collision|SetActorEnableCollision false)
  (Collision|SetCollisionEnabled (Variables|Default|GetForceTalkTrigger) "NoCollision"))

(event Collision|EventActorBeginOverlap
  (params (OtherActor :type Actor%20Object%20Reference)))

(event EventTick
  (params (DeltaSeconds :type Float%20%28single-precision%29)))

(fn ConstructionScript)

(fn MovetoNearestCompassSpawnPoint
  (Variables|Default|SetClosestDistance 999999999.0)
  (Variables|Default|SetClosestSpawnPoint 0)
  (bind _outactors (Actor|GetAllActorsOfClasswithTag "/Game/Grupp03_Test/Aimi/Blueprints/Objetcs/BP_TargetCompassBearer_Island4.BP_TargetCompassBearer_Island4_C" "CompassBearerSpawnPoint"))
  (for _array_element _outactors
    (if (< (Math|Vector|Distance(Vector) (Transformation|GetActorLocation _array_element) (Transformation|GetActorLocation (Game|Player|GetPlayerPawn 0))) (Variables|Default|GetClosestDistance))
      (Variables|Default|SetClosestDistance (Math|Vector|Distance(Vector) (Transformation|GetActorLocation _array_element) (Transformation|GetActorLocation (Game|Player|GetPlayerPawn 0))))
      (Variables|Default|SetClosestSpawnPoint _array_element)))
  (Utilities|IsValid (Variables|Default|GetClosestSpawnPoint)
    (:Is%20Valid
      (Transformation|SetActorLocation (Transformation|GetActorLocation (Variables|Default|GetClosestSpawnPoint)) false false)
      (Transformation|SetActorRotation (Transformation|GetActorRotation (Variables|Default|GetClosestSpawnPoint))))))