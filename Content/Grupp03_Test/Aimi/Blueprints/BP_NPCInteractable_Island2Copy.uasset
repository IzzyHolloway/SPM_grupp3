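; Island 2 NPC that walks along placed splines, first to a door and later out of a house.
; MoveToDoor starts the first walk; Tick advances the actor by speed and delta time along each spline, setting location and yaw.
; Tick polls the ProgressionManager for the Island2NPCExitedHouse flag to start the exit walk, which BeginPlay also starts if the flag is already set.
; Both spline components are cached from spline actors in the construction script.
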(event Custom|MoveToDoor
  ;[0.15 0.15 0.15 0.5] Start walking to the door
  (Variables|Default|SetIsWalkingToDoor true))

(event Collision|EventActorBeginOverlap
  (params (OtherActor :type Actor%20Object%20Reference)))

(event EventTick
  (params (DeltaSeconds :type Float%20%28single-precision%29))
  (if (Variables|Default|GetHasStartedExit)
    ;[0.15 0.15 0.15 0.5] 2. Walk out of the house
    (if (Variables|Default|GetIsWalkingOutOfHouse)
      ;[0.15 0.15 0.15 0.5] Update current distance: Add distance walked this frame
      (Variables|Default|SetCurrentDistance (+ (Variables|Default|GetCurrentDistance) (* (Variables|Default|GetSpeed) DeltaSeconds)))
      ;[0.15 0.15 0.15 0.5] Set new actor location: distance along spline
      (Transformation|SetActorLocation (Spline|GetLocationatDistanceAlongSpline (Variables|Default|GetSplinePart2) (Variables|Default|GetCurrentDistance) "World") false false)
      ;[0.15 0.15 0.15 0.5] Set new rotation: Not needed right now, since NPC looks the same from all sides
      (Transformation|SetActorRotation (Math|Rotator|MakeRotator 0.0 0.0 (- (.yaw (Spline|GetRotationatDistanceAlongSpline (Variables|Default|GetSplinePart2) (Variables|Default|GetCurrentDistance) "Local")) 9e+01)))
      ;[0.15 0.15 0.15 0.5] End walking if whole distances has been travelled
      (if (>= (Variables|Default|GetCurrentDistance) (Spline|GetSplineLength (Variables|Default|GetSplinePart2)))
        (Variables|Default|SetIsWalkingOutOfHouse false)))
    (else
      (Utilities|FlowControl|Sequence
        (:then_0
          ;[0.15 0.15 0.15 0.5] 1. Walk to the door
          (if (Variables|Default|GetIsWalkingToDoor)
            ;[0.15 0.15 0.15 0.5] Update current distance: Add distance walked this frame
            (Variables|Default|SetCurrentDistance (+ (Variables|Default|GetCurrentDistance) (* (Variables|Default|GetSpeed) DeltaSeconds)))
            ;[0.15 0.15 0.15 0.5] Set new actor location: distance along spline
            (Transformation|SetActorLocation (Spline|GetLocationatDistanceAlongSpline (Variables|Default|GetSplinePart1) (Variables|Default|GetCurrentDistance) "World") false false)
            ;[0.15 0.15 0.15 0.5] Set new rotation: Not needed right now, since NPC looks the same from all sides
            (Transformation|SetActorRotation (Math|Rotator|MakeRotator 0.0 0.0 (- (.yaw (Spline|GetRotationatDistanceAlongSpline (Variables|Default|GetSplinePart1) (Variables|Default|GetCurrentDistance) "Local")) 9e+01)))
            ;[0.15 0.15 0.15 0.5] End walking if whole distances has been travelled
            (if (>= (Variables|Default|GetCurrentDistance) (Spline|GetSplineLength (Variables|Default|GetSplinePart1)))
              (Variables|Default|SetIsWalkingToDoor false)
              ;;[0.15 0.15 0.15 0.5] Reset distance for walking along another spline later
              (Variables|Default|SetCurrentDistance 0.0))))
        (:then_1
          (bind _returnvalue (Actor|GetActorOfClass "/Script/SPM_grupp3.ProgressionManager"))
          (if (Class|ProgressionManager|HasFlag _returnvalue "Island2NPCExitedHouse")
            (Variables|Default|SetIsWalkingOutOfHouse true)
            (Variables|Default|SetHasStartedExit true)))))))

(event EventBeginPlay
  (bind _returnvalue (Actor|GetActorOfClass "/Script/SPM_grupp3.ProgressionManager"))
  (if (Class|ProgressionManager|HasFlag _returnvalue "Island2NPCExitedHouse")
    (Variables|Default|SetIsWalkingOutOfHouse true)
    (Variables|Default|SetHasStartedExit true)
    (else
      (Variables|Default|SetIsWalkingOutOfHouse false)
      (Variables|Default|SetHasStartedExit false))))

(event Input|KeyboardEvents|O
  (params (Key :type Key%20Structure :default "None"))
  ;[0.15 0.15 0.15 0.5] Only for debugging: Trigger walking when pressing debug key
  (:Pressed
    ;[0.15 0.15 0.15 0.5] Start walking out of the house
    (Variables|Default|SetIsWalkingOutOfHouse true)))

(fn ConstructionScript
  ;[0.15 0.15 0.15 0.5] Save spline components of spline actors
  (Variables|Default|SetSplinePart2 (Actor|GetComponentbyClass (Variables|Default|GetSplineActorPart2) "/Script/Engine.SplineComponent"))
  (Variables|Default|SetSplinePart1 (Actor|GetComponentbyClass (Variables|Default|GetSplineActorPart1) "/Script/Engine.SplineComponent")))