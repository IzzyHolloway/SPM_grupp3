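; BP_Gate is a gate that opens once the Island3PadlockSolved flag is set, then sends the player to Level 2.
; Tick polls the ProgressionManager for the flag and interpolates the gate from its start position to a hard-coded world height.
; A DoOnce plays the gate sound and a media cutscene in a widget, then travels via the game instance after a fixed delay matched by hand to the video length.
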(event EventBeginPlay
  (bind _returnvalue (Transformation|GetActorLocation))
  (Variables|Default|SetClosedLocation (Transformation|GetActorLocation))
  (Variables|Default|SetOpenLocation (Math|Vector|MakeVector (.x _returnvalue) (.y _returnvalue) -3.5e+03)))

(event Collision|EventActorBeginOverlap
  (params (OtherActor :type Actor%20Object%20Reference)))

(event EventTick
  (params (DeltaSeconds :type Float%20%28single-precision%29))
  (bind _returnvalue (Actor|GetActorOfClass "/Script/SPM_grupp3.ProgressionManager"))
  (if (Class|ProgressionManager|HasFlag _returnvalue "Island3PadlockSolved")
    (Transformation|SetActorLocation (Math|Interpolation|VInterpTo (Transformation|GetActorLocation) (Variables|Default|GetOpenLocation) DeltaSeconds 4.0) false false)
    (Utilities|FlowControl|DoOnce false
      (:Completed
        (Class|FMODBlueprintStatics|PlayEventatLocation "/Game/FMOD/Events/Gate.Gate" (Math|Conversions|ToTransform(Vector) (Transformation|GetActorLocation)))
        (Media|MediaPlayer|OpenSource (Variables|Default|GetMyMediaPlayer) "/Game/Movies/Sequence01.Sequence01")
        ;[0.15 0 0.002878 0.5] Change the WBP to the cutscene
        (bind _returnvalue_2 (UserInterface|CreateWidget "/Game/Grupp03_Test/Izzy/WBP_Cutscene.WBP_Cutscene_C"))
        (UserInterface|Viewport|AddtoViewport _returnvalue_2 0)
        ;[0.15 0.001527 0 0.5] Change the duration depending on the length of the cutscene
        (Utilities|FlowControl|Delay 7.0)
        (Widget|RemovefromParent _returnvalue_2)
        (bind _aslittle_lost_game_instance (Utilities|Casting|CastToLittleLost_GameInstance (Game|GetGameInstance)))
        (Class|LittleLostGameInstance|TraveltoLevel _aslittle_lost_game_instance "LVL_ALittleLost_Level2" false)))))

(fn ConstructionScript)