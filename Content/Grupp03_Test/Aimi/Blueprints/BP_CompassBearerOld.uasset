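; Compass Bearer NPC that stays hidden without collision until the story progression makes it appear.
; A looping timer polls BP_ProgressionManager for the CompassBearerSpawned flag, then clears itself once the bearer appears.
; On appearing, it snaps to the tagged BP_TargetCompassBearer_Island4 spawn point nearest the player and becomes visible.
; A trigger box starts its auto dialogue through BP_DialogueManager the first time CharacterAimi overlaps it.
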(event OnComponentBeginOverlap(DialogueTriggerBox)
  (params (OverlappedComponent :type Primitive%20Component%20Object%20Reference) (OtherActor :type Actor%20Object%20Reference) (OtherComp :type Primitive%20Component%20Object%20Reference) (OtherBodyIndex :type Integer) (bFromSweep :type Boolean) (SweepResult :type Hit%20Result%20Structure%20%28by%20ref%29))
  (Utilities|Casting|CastToCharacterAimi OtherActor)
  (if (not (Variables|Default|GetbDialogueTriggered))
    (Variables|Default|SetbDialogueTriggered true)
    (bind _returnvalue (Actor|GetActorOfClass "/Game/Grupp03_Test/Aimi/Blueprints/Managers/BP_DialogueManager.BP_DialogueManager_C"))
    (Class|DialogueManager|StartDialoguefromDataAsset _returnvalue (Variables|Default|GetAutoDialogueData))))

(event Custom|AppearCompassBearer
  (CallFunction|MovetoNearestCompassSpawnPoint)
  (Rendering|SetActorHiddenInGame false)
  (Collision|SetActorEnableCollision true)
  (Variables|Default|SetbHasAppeared true)
  (Development|PrintString "Compass Bearer appeared"))

(event Custom|CheckCompassBearerSpawn
  (if (not (Variables|Default|GetbHasAppeared))
    (bind _returnvalue (Actor|GetActorOfClass "/Game/Grupp03_Test/Aimi/Blueprints/Managers/BP_ProgressionManager.BP_ProgressionManager_C"))
    (if (Class|ProgressionManager|HasFlag _returnvalue "CompassBearerSpawned")
      (CallFunction|AppearCompassBearer)
      (Utilities|Time|ClearandInvalidateTimerbyHandle (stale EventBeginPlay _returnvalue)))))

(event Custom|TriggerCompassBearerSequence
  (if true
    _))

(event EventBeginPlay
  (Rendering|SetActorHiddenInGame true)
  (Collision|SetActorEnableCollision false)
  (Variables|Default|SetbHasAppeared false)
  (bind _returnvalue (Utilities|Time|SetTimerbyEvent (delegate Custom|CheckCompassBearerSpawn) 0.25 true)))

(event Collision|EventActorBeginOverlap
  (params (OtherActor :type Actor%20Object%20Reference)))

(event EventTick
  (params (DeltaSeconds :type Float%20%28single-precision%29)))

(fn ConstructionScript)

(fn MovetoNearestCompassSpawnPoint
  (Variables|Default|SetClosestDistance 999999999.0)
  (Variables|Default|SetClosestSpawnPoint 0)
  (bind _outactors (Actor|GetAllActorsOfClasswithTag "/Game/Grupp03_Test/Aimi/Blueprints/Objetcs/BP_TargetCompassBearer_Island4.BP_TargetCompassBearer_Island4_C" "CompassBearerSpawnPoint"))
  (for _array_element _outactors
    (if (< (Math|Vector|Distance(Vector) (Transformation|GetActorLocation _array_element) (Transformation|GetActorLocation (Game|Player|GetPlayerPawn 0))) (Variables|Default|GetClosestDistance))
      (Variables|Default|SetClosestDistance (Math|Vector|Distance(Vector) (Transformation|GetActorLocation _array_element) (Transformation|GetActorLocation (Game|Player|GetPlayerPawn 0))))
      (Variables|Default|SetClosestSpawnPoint _array_element)))
  (Utilities|IsValid (Variables|Default|GetClosestSpawnPoint)
    (:Is%20Valid
      (Transformation|SetActorLocation (Transformation|GetActorLocation (Variables|Default|GetClosestSpawnPoint)) false false)
      (Transformation|SetActorRotation (Transformation|GetActorRotation (Variables|Default|GetClosestSpawnPoint))))))