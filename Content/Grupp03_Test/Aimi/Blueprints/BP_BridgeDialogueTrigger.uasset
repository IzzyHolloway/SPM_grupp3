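; BP_BridgeDialogueTrigger is a one-shot trigger volume that plays an intro dialogue when the player character enters it.
; Its Box overlap casts to BP_CharacterSpeltest1, passes a DoOnce, then finds BP_DialogueManager through GetActorOfClass.
; It sends the lines of the first IntroDialogueData entry, using StartDialogueWithFlag when that entry sets a flag on end, otherwise StartDialogue.
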(event OnComponentBeginOverlap(Box)
  (params (OverlappedComponent :type Primitive%20Component%20Object%20Reference) (OtherActor :type Actor%20Object%20Reference) (OtherComp :type Primitive%20Component%20Object%20Reference) (OtherBodyIndex :type Integer) (bFromSweep :type Boolean) (SweepResult :type Hit%20Result%20Structure%20%28by%20ref%29))
  (bind _introdialoguedata (Variables|Default|GetIntroDialogueData))
  (bind _dialogueentries (Variables|/Script/SPM_grupp3.DialogueDataAsset|GetDialogueEntries _introdialoguedata))
  (bind _output (Utilities|Array|Get(acopy) _dialogueentries))
  (bind (_dialogueid _requiredflags _blockedflags _dialoguelines _rawdialogueimporttext _bsetflagondialogueend _flagtosetondialogueend) (Utilities|Struct|BreakDialogueEntry _output))
  (Utilities|Casting|CastToBP_CharacterSpeltest1 OtherActor)
  (Utilities|FlowControl|DoOnce false
    (:Completed
      (bind _returnvalue (Actor|GetActorOfClass "/Game/Grupp03_Test/Aimi/Blueprints/BP_DialogueManager.BP_DialogueManager_C"))
      (if _bsetflagondialogueend
        (Class|DialogueManager|StartDialoguewithFlag _returnvalue _dialoguelines _flagtosetondialogueend)
        (else
          (Class|DialogueManager|StartDialogue _returnvalue _dialoguelines))))))

(fn ConstructionScript)