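; Engine interactable that runs the game's ending sequence once the engine is installed.
; Installation sets a lighthouse progression flag, plays the camera director's lighthouse cutscene and starts a dialogue.
; When dialogue ends, it locks player input and plays a media cutscene in a widget with a hold-to-skip prompt.
; A hardcoded delay or completed skip triggers a guarded finish that restores input and opens the main menu.
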(event Custom|FinishTestCutscene
  (bind _returnvalue (Game|GetPlayerController 0))
  (bind _returnvalue_2 (Game|GetPlayerController 0))
  (bind _endcutscenewidget (Variables|Default|GetEndCutsceneWidget))
  (bind _skippromptwidget (Variables|Default|GetSkipPromptWidget))
  (if (not (Variables|Default|GetbCutsceneFinished))
    (Variables|Default|SetbCutsceneFinished true)
    (Variables|Default|SetbCutsceneActive false)
    (Media|MediaPlayer|Close (Variables|Default|GetStart%20Cutscene%20Media%20Player) :!class /Script/MediaAssets.MediaPlayer)
    (Utilities|IsValid _endcutscenewidget
      (:Is%20Valid
        (Widget|RemovefromParent _endcutscenewidget)
        (Utilities|IsValid _skippromptwidget
          (:Is%20Valid
            (Widget|RemovefromParent _skippromptwidget)
            (Input|SetIgnoreMoveInput _returnvalue false)
            (Input|SetIgnoreLookInput _returnvalue false)
            (Input|SetInputModeGameOnly _returnvalue_2 false)
            (Variables|/Script/Engine.PlayerController|SetbShowMouseCursor _returnvalue_2 false)
            (Development|PrintString (Utilities|GetDisplayName (Pawn|GetControlledPawn _returnvalue_2)))
            (Game|OpenLevel(byName) "L_MainMenu")))))))

(event Custom|StartEndWidgetCutscene
  (bind _returnvalue (Game|GetPlayerController 0))
  (bind _returnvalue_2 (UserInterface|CreateWidget "/Game/Blueprints/WBP/CutScenes/WBP_EndCutscene.WBP_EndCutscene_C"))
  (UserInterface|Viewport|AddtoViewport _returnvalue_2 0)
  (Input|EnableInput _returnvalue)
  (Input|SetInputModeGameOnly _returnvalue false)
  (Input|SetIgnoreMoveInput _returnvalue true)
  (Input|SetIgnoreLookInput _returnvalue true)
  (Variables|/Script/Engine.PlayerController|SetbShowMouseCursor _returnvalue false)
  (Utilities|FlowControl|DoOnce false
    (:Completed
      (bind _returnvalue_3 (UserInterface|CreateWidget "/Game/Blueprints/WBP/CutScenes/WBP_EndCutscene.WBP_EndCutscene_C"))
      (bind _output_get (Variables|Default|SetEndCutsceneWidget _returnvalue_3))
      (UserInterface|Viewport|AddtoViewport _output_get 0)
      (bind _returnvalue_4 (UserInterface|CreateWidget "/Game/Blueprints/WBP/UI_Overlay/WBP_SkipPrompt.WBP_SkipPrompt_C"))
      (bind _output_get_2 (Variables|Default|SetSkipPromptWidget _returnvalue_4))
      (EventDispatchers|BindEventtoOnSkipCompleted _output_get_2 (delegate Custom|FinishTestCutscene))
      (UserInterface|Viewport|AddtoViewport _output_get_2 10)
      (Variables|Default|SetbCutsceneActive true)
      (Variables|Default|SetbCutsceneFinished false)
      (Media|MediaPlayer|OpenSource (Variables|Default|GetStart%20Cutscene%20Media%20Player) "/Game/Movies/Cutscene3.Cutscene3")
      (Utilities|FlowControl|Delay 0.4)
      (Media|MediaPlayer|Play (Variables|Default|GetStart%20Cutscene%20Media%20Player) :!class /Script/MediaAssets.MediaPlayer)
      ;[0.15 0.001527 0 0.5] Change the duration depending on the length of the cutscene
      (Utilities|FlowControl|Delay 56.0)
      (CallFunction|FinishTestCutscene))))

(event Input|EnhancedActionEvents|EnhancedInputActionIA_DialogueAdvance
  (params (ActionValue :type Boolean) (ElapsedSeconds :type Float%20%28double-precision%29) (TriggeredSeconds :type Float%20%28double-precision%29) (InputAction :type Input%20Action%20Object%20Reference :default "/Game/Input/Actions/IA_DialogueAdvance.IA_DialogueAdvance"))
  (bind _skippromptwidget (Variables|Default|GetSkipPromptWidget))
  (bind _skippromptwidget_2 (Variables|Default|GetSkipPromptWidget))
  (:Started
    (Development|PrintString "START SKIP HOLD")
    (if (Variables|Default|GetbCutsceneActive)
      (Utilities|IsValid _skippromptwidget
        (:Is%20Valid
          (Default|StartSkipHold _skippromptwidget)))))
  (:Canceled
    (if (Variables|Default|GetbCutsceneActive) :!label _label
      (Utilities|IsValid _skippromptwidget_2
        (:Is%20Valid
          (Default|StopSkipHold _skippromptwidget_2)))))
  (:Completed
    (goto _label)))

(event EventBeginPlay)

(event Collision|EventActorBeginOverlap
  (params (OtherActor :type Actor%20Object%20Reference)))

(event EventTick
  (params (DeltaSeconds :type Float%20%28single-precision%29)))

(event EventOnEngineInstalled
  (bind _returnvalue (Actor|GetActorOfClass "/Game/Grupp03_Test/Aimi/Blueprints/Managers/BP_ProgressionManager.BP_ProgressionManager_C"))
  (Class|ProgressionManager|AddFlag _returnvalue "LighthouseLightCutscenePlayed")
  (bind _returnvalue_2 (Actor|GetActorOfClass "/Game/Grupp03_Test/Madde/Blueprints/BP_CameraDirector.BP_CameraDirector_C"))
  (Default|PlayLighthouseCutscene _returnvalue_2)
  (Utilities|FlowControl|Delay 1.5)
  (bind _returnvalue_3 (Actor|GetActorOfClass "/Game/Grupp03_Test/Aimi/Blueprints/Managers/BP_DialogueManager.BP_DialogueManager_C"))
  (EventDispatchers|BindEventtoOnDialogueEnded _returnvalue_3 (delegate Custom|StartEndWidgetCutscene))
  (Class|DialogueManager|StartDialoguefromDataAsset _returnvalue_3 "/Game/Grupp03_Test/Aimi/DataAssets/DA_TheLostOne.DA_TheLostOne"))

(fn ConstructionScript)

(fn FinishLevel2Cutscene)