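; Player controller Blueprint that toggles a pause menu from the IA_Pause Enhanced Input action.
; BeginPlay sets game-only input.
; Pausing lazily creates and caches a WBP_PauseMenu widget, adds it to the player screen, pauses the game, and switches to game-and-UI input with the cursor shown.
; Unpausing removes the widget, resumes the game, and restores game-only input with the cursor hidden.
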(event Input|EnhancedActionEvents|EnhancedInputActionIA_Pause
  (params (ActionValue :type Boolean) (ElapsedSeconds :type Float%20%28double-precision%29) (TriggeredSeconds :type Float%20%28double-precision%29) (InputAction :type Input%20Action%20Object%20Reference :default "/Game/Input/Actions/IA_Pause.IA_Pause"))
  (:Started
    (if (Game|IsGamePaused)
      (Widget|RemovefromParent (Variables|Default|GetNewerPauseRef))
      (Game|SetGamePaused false)
      (Input|SetInputModeGameOnly self false)
      (Variables|Default|SetbShowMouseCursor false)
      (else
        (Utilities|IsValid (Variables|Default|GetNewerPauseRef)
          (:Is%20Valid
            _)
          (:Is%20Not%20Valid
            (bind _returnvalue (UserInterface|CreateWidget "/Game/Blueprints/WBP/Menus/WBP_PauseMenu.WBP_PauseMenu_C"))
            (bind _output_get (Variables|Default|SetNewerPauseRef _returnvalue))))
        (UserInterface|Viewport|AddtoPlayerScreen _output_get)
        (Game|SetGamePaused true)
        (Input|SetInputModeGameandUI self (Variables|Default|GetNewerPauseRef) "DoNotLock" true false)
        (Variables|Default|SetbShowMouseCursor true)))))

(event EventBeginPlay
  (Input|SetInputModeGameOnly self false))

(fn ConstructionScript)