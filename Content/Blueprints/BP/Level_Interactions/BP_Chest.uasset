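; Interactable chest that highlights via custom depth and accepts interact input while an actor overlaps its InteractionSphere.
; IA_Interact drives the OpenLid timeline, rotating the lid hinge and raising the linked hidden pickup, or reversing both.
; Opening requires a valid pickup, which becomes visible and collidable shortly after the timeline finishes.
; Tick closes an open chest automatically once that pickup is no longer valid.
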(event OnComponentBeginOverlap(InteractionSphere)
  (params (OverlappedComponent :type Primitive%20Component%20Object%20Reference) (OtherActor :type Actor%20Object%20Reference) (OtherComp :type Primitive%20Component%20Object%20Reference) (OtherBodyIndex :type Integer) (bFromSweep :type Boolean) (SweepResult :type Hit%20Result%20Structure%20%28by%20ref%29))
  ;[0.15 0.15 0.15 0.5] Show/hide the interaction prompt when the player enters/leaves the InteractionSphere.
  ; Also enables Enhanced Input on the chest so outline only listens while in range.
  (Rendering|SetRenderCustomDepth (Variables|Default|GetBody) true)
  (Rendering|SetRenderCustomDepth (Variables|Default|GetLid) true)
  (Input|EnableInput (Game|GetPlayerController 0)))

(event OnComponentEndOverlap(InteractionSphere)
  (params (OverlappedComponent :type Primitive%20Component%20Object%20Reference) (OtherActor :type Actor%20Object%20Reference) (OtherComp :type Primitive%20Component%20Object%20Reference) (OtherBodyIndex :type Integer))
  ;[0.15 0.15 0.15 0.5] Show/hide the interaction prompt when the player enters/leaves the InteractionSphere.
  ; Also enables Enhanced Input on the chest so outline only listens while in range.
  (Rendering|SetRenderCustomDepth (Variables|Default|GetBody) false)
  (Rendering|SetRenderCustomDepth (Variables|Default|GetLid) false)
  (Input|DisableInput (Game|GetPlayerController 0)))

(event Input|EnhancedActionEvents|EnhancedInputActionIA_Interact
  (params (ActionValue :type Boolean) (ElapsedSeconds :type Float%20%28double-precision%29) (TriggeredSeconds :type Float%20%28double-precision%29) (InputAction :type Input%20Action%20Object%20Reference :default "/Game/Input/Actions/IA_Interact.IA_Interact"))
  (bind _my_hidden_pickup (Variables|Default|GetMy%20Hidden%20Pickup))
  (bind _my_hidden_pickup_2 (Variables|Default|GetMy%20Hidden%20Pickup))
  ;[0.15 0.15 0.15 0.5] Open/close logic — pressing IA_Interact plays the OpenLid timeline forward (opens lid and lifts the hidden pickup up) or in reverse (closes lid). State tracked by bIsOpen, final state set after a short delay when the timeline finishes.
  (:Started
    (if (Variables|Default|GetbIsOpen)
      (Variables|Default|SetbIsOpen false)
      (bind (_direction _lidrotation _pickupheight) (Timeline|OpenLid Reverse)
        (:Update
          (Transformation|SetRelativeRotation (Variables|Default|GetLidHinge) (Math|Rotator|MakeRotator _lidrotation 0.0 0.0) false false)
          (Utilities|IsValid _my_hidden_pickup
            (:Is%20Valid
              (Transformation|SetActorLocation _my_hidden_pickup (+ (Variables|Default|GetPickupStartLocation) (Math|Vector|MakeVector 0.0 0.0 _pickupheight)) false false))))
        (:Finished
          (if (not (Variables|Default|GetbIsOpen))
            (Utilities|FlowControl|Delay 0.7)
            (Variables|Default|SetbIsOpen true)
            (Utilities|IsValid _my_hidden_pickup_2
              (:Is%20Valid
                (Rendering|SetActorHiddenInGame _my_hidden_pickup_2 false)
                (Collision|SetActorEnableCollision _my_hidden_pickup_2 true))))))
      (else
        (Utilities|IsValid (Variables|Default|GetMy%20Hidden%20Pickup)
          (:Is%20Valid
            (Collision|SetActorEnableCollision false)
            (Variables|Default|SetPickupStartLocation (Transformation|GetActorLocation (Variables|Default|GetMy%20Hidden%20Pickup)))
            (Timeline|OpenLid Play)))))))

(event EventTick
  (params (DeltaSeconds :type Float%20%28single-precision%29))
  (bind _my_hidden_pickup (Variables|Default|GetMy%20Hidden%20Pickup))
  (bind _my_hidden_pickup_2 (Variables|Default|GetMy%20Hidden%20Pickup))
  ;[0.15 0.15 0.15 0.5] Open/close logic — pressing IA_Interact plays the OpenLid timeline forward (opens lid and lifts the hidden pickup up) or in reverse (closes lid). State tracked by bIsOpen, final state set after a short delay when the timeline finishes.
  (Utilities|IsValid (Variables|Default|GetMy%20Hidden%20Pickup)
    (:Is%20Not%20Valid
      (if (Variables|Default|GetbIsOpen)
        (Variables|Default|SetbIsOpen false)
        (bind (_direction _lidrotation _pickupheight) (Timeline|OpenLid Reverse)
          (:Update
            (Transformation|SetRelativeRotation (Variables|Default|GetLidHinge) (Math|Rotator|MakeRotator _lidrotation 0.0 0.0) false false)
            (Utilities|IsValid _my_hidden_pickup
              (:Is%20Valid
                (Transformation|SetActorLocation _my_hidden_pickup (+ (Variables|Default|GetPickupStartLocation) (Math|Vector|MakeVector 0.0 0.0 _pickupheight)) false false))))
          (:Finished
            (if (not (Variables|Default|GetbIsOpen))
              (Utilities|FlowControl|Delay 0.7)
              (Variables|Default|SetbIsOpen true)
              (Utilities|IsValid _my_hidden_pickup_2
                (:Is%20Valid
                  (Rendering|SetActorHiddenInGame _my_hidden_pickup_2 false)
                  (Collision|SetActorEnableCollision _my_hidden_pickup_2 true))))))))))

(fn ConstructionScript)

(fn LookatActor
  (return ""))