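; BP_PanelInteractable is an interactable panel that opens a UI widget when the player interacts with it.
; OnInteract, guarded by IsOpen, creates WBP_PanelInteractable with a back-reference to the panel, focuses it in Game and UI input mode, locks BP_CharacterSpeltest1's movement and shows the mouse.
; CloseInteraction removes the widget, unlocks movement, hides the mouse and clears IsOpen.
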(event EventOnInteract
  (if (not (Variables|Default|GetIsOpen))
    (Variables|Default|SetIsOpen true)
    (bind _returnvalue (UserInterface|CreateWidget "/Game/Blueprints/WBP/Puzzles/WBP_PanelInteractable.WBP_PanelInteractable_C"))
    (Variables|/Game/Blueprints/WBP/Puzzles/WBP_PanelInteractable.WBP_PanelInteractable_C|SetPanelRef _returnvalue self)
    (UserInterface|Viewport|AddtoViewport _returnvalue 100)
    (Input|SetInputModeGameandUI (Game|GetPlayerController 0) _returnvalue "DoNotLock" true false)
    (bind _returnvalue_2 (Actor|GetActorOfClass "/Game/Characters/BP_CharacterSpeltest1.BP_CharacterSpeltest1_C"))
    (Class|CharacterAimi|SetMovementLocked _returnvalue_2 true)
    (CallFunction|ShowMouse _returnvalue)))

(event EventCloseInteraction
  (Widget|RemovefromParent (Variables|Default|GetPanelInteractable))
  (bind _returnvalue (Actor|GetActorOfClass "/Game/Characters/BP_CharacterSpeltest1.BP_CharacterSpeltest1_C"))
  (Class|CharacterAimi|SetMovementLocked _returnvalue false)
  (CallFunction|HideMouse)
  (Variables|Default|SetIsOpen false))

(fn ConstructionScript)