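; Stone actor for the island 3 stone puzzle (Puzzle 4), with a sphere mesh and point light that animate vertically.
; MoveStoneDown plays a timeline that lowers both by StoneOffset and drives light intensity, then immediately reverses it on finish.
; CompletePuzzle uses a second timeline to move both down ten times that offset.
; StoneAnimation is an interpolation-based alternative with a debug print, not called within this Blueprint.
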(event Custom|CompletePuzzle
  (bind _alpha (Timeline|Puzzle%20Complete%20Timeline Play)
    (:Update
      (Transformation|SetRelativeLocation (Variables|Default|GetSphere) (Math|Vector|MakeVector 0.0 0.0 (* _alpha (* (Variables|Default|GetStone%20Offset) -1e+01))) false false)
      (Transformation|SetRelativeLocation (Variables|Default|GetPointLight) (Math|Vector|MakeVector 0.0 0.0 (* _alpha (* (Variables|Default|GetStone%20Offset) -1e+01))) false false))))

(event Custom|MoveStoneDown
  (bind _pointlight (Variables|Default|GetPointLight))
  ;[0.15 0.15 0.15 0.5] Stone Animation for Stone Puzzle Island 3 (Puzzle 4)
  (bind (_direction _stone_offset_alpha _light_intensity) (Timeline|StoneTimeline Play)
    (:Update
      (Transformation|SetRelativeLocation (Variables|Default|GetSphere) (Math|Vector|MakeVector 0.0 0.0 (* _stone_offset_alpha (* (Variables|Default|GetStone%20Offset) -1.0))) false false)
      (Transformation|SetRelativeLocation _pointlight (Math|Vector|MakeVector 0.0 0.0 (* _stone_offset_alpha (* (Variables|Default|GetStone%20Offset) -1.0))) false false)
      (Rendering|Components|Light|SetIntensity _pointlight (* _light_intensity (Variables|Default|GetLight%20Intensity))))
    (:Finished
      (switch Utilities|FlowControl|Switch|SwitchonETimelineDirection _direction
        (:Forward
          (CallFunction|MoveStoneUpwards)
          (Utilities|FlowControl|Delay 2.5))
        (:Backward
          (Utilities|FlowControl|Delay 2.0))))))

(event Custom|MoveStoneUpwards
  (bind _pointlight (Variables|Default|GetPointLight))
  ;[0.15 0.15 0.15 0.5] Stone Animation for Stone Puzzle Island 3 (Puzzle 4)
  (bind (_direction _stone_offset_alpha _light_intensity) (Timeline|StoneTimeline Reverse)
    (:Update
      (Transformation|SetRelativeLocation (Variables|Default|GetSphere) (Math|Vector|MakeVector 0.0 0.0 (* _stone_offset_alpha (* (Variables|Default|GetStone%20Offset) -1.0))) false false)
      (Transformation|SetRelativeLocation _pointlight (Math|Vector|MakeVector 0.0 0.0 (* _stone_offset_alpha (* (Variables|Default|GetStone%20Offset) -1.0))) false false)
      (Rendering|Components|Light|SetIntensity _pointlight (* _light_intensity (Variables|Default|GetLight%20Intensity))))
    (:Finished
      (switch Utilities|FlowControl|Switch|SwitchonETimelineDirection _direction
        (:Forward
          (CallFunction|MoveStoneUpwards)
          (Utilities|FlowControl|Delay 2.5))
        (:Backward
          (Utilities|FlowControl|Delay 2.0))))))

(event EventBeginPlay)

(event Collision|EventActorBeginOverlap
  (params (OtherActor :type Actor%20Object%20Reference)))

(event EventTick
  (params (DeltaSeconds :type Float%20%28single-precision%29)))

(fn ConstructionScript)

(fn StoneAnimation
  (bind _returnvalue (Transformation|GetActorLocation))
  (bind _returnvalue_2 (Utilities|Time|GetWorldDeltaSeconds))
  (bind _stone_offset (Variables|Default|GetStone%20Offset))
  (bind (_x _y _z) (Math|Vector|BreakVector _returnvalue))
  (bind _returnvalue_3 (- _z _stone_offset))
  (bind _returnvalue_4 (Math|Vector|MakeVector _x _y _returnvalue_3))
  (bind _returnvalue_5 (Math|Interpolation|VInterpTo _returnvalue _returnvalue_4 _returnvalue_2 5.0))
  (Development|PrintString (Utilities|String|ToString(Vector) _returnvalue_4))
  (Transformation|SetActorLocation _returnvalue_5 false false)
  (Rendering|Components|Light|SetIntensity (Variables|Default|GetPointLight) (Math|Interpolation|FInterpTo 0.0 (Variables|Default|GetLight%20Intensity) (Utilities|Time|GetWorldDeltaSeconds) 5.0))
  (Transformation|SetActorLocation (Math|Interpolation|VInterpTo _returnvalue_5 (Transformation|GetActorLocation) (Utilities|Time|GetWorldDeltaSeconds) 5.0) false false)
  (Rendering|Components|Light|SetIntensity (Variables|Default|GetPointLight) (Math|Interpolation|FInterpTo (Variables|Default|GetLight%20Intensity) 0.0 (Utilities|Time|GetWorldDeltaSeconds) 5.0))
  (return))