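; BPC_Interaction is an actor component that lets its owner detect and use nearby Interactable actors.
; Each tick, a zero-length sphere trace at the owner's location stores the hit actor if it implements Interactable, otherwise clears it.
; The actor's look-at message feeds a WB_InteractNotify widget created on BeginPlay, which is blanked when nothing qualifies.
; IA_Interact sends InteractWithMessage to the stored actor, passing the owner.
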(event Input|EnhancedActionEvents|EnhancedInputActionIA_Interact
  (params (ActionValue :type Boolean) (ElapsedSeconds :type Float%20%28double-precision%29) (TriggeredSeconds :type Float%20%28double-precision%29) (InputAction :type Input%20Action%20Object%20Reference :default "/Game/Input/Actions/IA_Interact.IA_Interact"))
  (:Started
    (Utilities|IsValid (Variables|Default|GetLookedAtActor)
      (:Is%20Valid
        (Class|Interactable|Interactwith(Message) (Variables|Default|GetLookedAtActor) (Components|GetOwner))))))

(event EventBeginPlay
  (CallFunction|CreateInteractionWidget))

(event EventTick
  (params (DeltaSeconds :type Float%20%28single-precision%29))
  (CallFunction|InteractTrace))

(fn CreateInteractionWidget
  (bind _returnvalue (UserInterface|CreateWidget "/Game/Blueprints/WBP/UI_Overlay/WB_InteractNotify.WB_InteractNotify_C"))
  (bind _output_get (Variables|Default|SetInteractNotifyWidget _returnvalue))
  (UserInterface|Viewport|AddtoViewport _output_get 0))

(fn InteractTrace
  (bind _returnvalue (Components|GetOwner))
  (bind _returnvalue_2 (Transformation|GetActorLocation _returnvalue))
  (bind (_outhit _returnvalue_3) (Collision|SphereTraceByChannel _returnvalue_2 _returnvalue_2 8e+01 "TraceTypeQuery3" false 0 "None"))
  (if _returnvalue_3
    (if (Utilities|DoesObjectImplementInterface (.HitActor (Collision|BreakHitResult _outhit)) "/Script/SPM_grupp3.Interactable")
      (bind _output_get (Variables|Default|SetLookedAtActor (.HitActor (Collision|BreakHitResult _outhit))))
      (bind _returnvalue_4 (Class|Interactable|LookatActor(Message) _output_get))
      (Default|UpdateInteractNotify (Variables|Default|GetInteractNotifyWidget) _returnvalue_4)
      (else
        (Variables|Default|SetLookedAtActor 0)
        (Default|UpdateInteractNotify (Variables|Default|GetInteractNotifyWidget))))
    (else
      (Variables|Default|SetLookedAtActor 0)
      (Default|UpdateInteractNotify (Variables|Default|GetInteractNotifyWidget)))))