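; Water monster AI that threatens the player's boat through two events, moving a particle body along timeline lerps.
; AIHitEvent, gated by a ProgressionManager flag, plays sound, camera shake and rumble, then charges from a randomized point ahead of the boat toward its live position, just below it.
; On arrival it shoves the boat with an impulse if possessed.
; AIShowToPlayerEvent glides it between the current event trigger's start and end positions.
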(event Custom|AI%20Hit%20Event
  (bind _returnvalue (Actor|GetActorOfClass "/Script/SPM_grupp3.ProgressionManager"))
  (if (Class|ProgressionManager|HasFlag _returnvalue "TalkedToListenerAfterPuzzle")
    (Audio|PlaySoundatLocation "/Game/Audio/water/AI_Monster/SC_SFX_AIMonster.SC_SFX_AIMonster" (Transformation|GetActorLocation) "0, 0, 0" 1.0 1.0 0.0 0 0 0 0)
    (Development|PrintString "Hello")
    (Components|Activation|Activate (Variables|Default|GetParticelBody) false)
    (bind _returnvalue_2 (Actor|GetActorOfClass "/Game/Blueprints/BP/Boat/BP_Boat_Functionality.BP_Boat_Functionality_C"))
    (Variables|Default|SetBoatFunctionality _returnvalue_2)
    (Default|CameraShake (Variables|Default|GetBoatFunctionality))
    (Game|Feedback|PlayDynamicForceFeedback (Game|GetPlayerController 0) 0.4 0.2 true true true true)
    (Variables|Default|SetStartLocation (Math|Vector|MakeVector (.X (Math|Vector|BreakVector (+ (* (Math|Vector|RotateVector (Transformation|GetActorForwardVector (Variables|Default|GetBoatFunctionality)) (Math|Rotator|MakeRotator 0.0 0.0 (Math|Random|RandomFloatinRange -45.0 45.0))) 3e+03) (Transformation|GetActorLocation (Variables|Default|GetBoatFunctionality))))) (.Y (Math|Vector|BreakVector (+ (* (Math|Vector|RotateVector (Transformation|GetActorForwardVector (Variables|Default|GetBoatFunctionality)) (Math|Rotator|MakeRotator 0.0 0.0 (Math|Random|RandomFloatinRange -45.0 45.0))) 3e+03) (Transformation|GetActorLocation (Variables|Default|GetBoatFunctionality))))) (- (.Z (Math|Vector|BreakVector (+ (* (Math|Vector|RotateVector (Transformation|GetActorForwardVector (Variables|Default|GetBoatFunctionality)) (Math|Rotator|MakeRotator 0.0 0.0 (Math|Random|RandomFloatinRange -45.0 45.0))) 3e+03) (Transformation|GetActorLocation (Variables|Default|GetBoatFunctionality))))) 1e+02)))
    (Variables|Default|SetBoatStartLocation (Transformation|GetActorLocation (Variables|Default|GetBoatFunctionality)))
    (bind _alpha (Timeline|AIWaterTimeline PlayFromStart)
      (:Update
        (Transformation|SetActorLocation (Math|Vector|Lerp(Vector) (Variables|Default|GetStartLocation) (Math|Vector|MakeVector (.X (Math|Vector|BreakVector (Transformation|GetActorLocation (Variables|Default|GetBoatFunctionality)))) (.Y (Math|Vector|BreakVector (Transformation|GetActorLocation (Variables|Default|GetBoatFunctionality)))) (- (.Z (Math|Vector|BreakVector (Transformation|GetActorLocation (Variables|Default|GetBoatFunctionality)))) 1e+02)) _alpha) false true))
      (:Finished
        ;[0.15 0.15 0.15 0.5] Pushing the player if it is in the boat
        (if (Variables|/Game/Blueprints/BP/Boat/BP_Boat_Functionality.BP_Boat_Functionality_C|GetPossessed (Variables|Default|GetBoatFunctionality))
          (Audio|PlaySoundatLocation "/Game/Audio/water/AI_Monster/S_SFX_BoatHit.S_SFX_BoatHit" (Transformation|GetActorLocation) "0, 0, 0" 1.0 1.0 0.0 0 0 0 0)
          (Physics|AddImpulse (Variables|/Script/SPM_grupp3.BoatFunctionality|GetCollisionComponent (Variables|Default|GetBoatFunctionality)) (* (Variables|Default|GetPushPower) (Math|Vector|GetUnitDirection(Vector) (Variables|Default|GetStartLocation) (Transformation|GetActorLocation))) "None" true))
        (Components|Activation|Deactivate (Variables|Default|GetParticelBody))))))

(event Custom|AI%20Show%20To%20Player%20Event
  (bind _current_event_trigger (Variables|Default|GetCurrent%20Event%20Trigger))
  (bind _current_event_trigger_2 (Variables|Default|GetCurrent%20Event%20Trigger))
  (bind _startposition (Variables|/Game/Blueprints/BP/AI/BP_WaterAIEventTrigger.BP_WaterAIEventTrigger_C|GetStartPosition _current_event_trigger))
  (Components|Activation|Activate (Variables|Default|GetParticelBody) false)
  (Transformation|SetActorLocation _startposition false true)
  (Development|PrintString (Utilities|String|ToString(Vector) _startposition))
  (bind _alpha (Timeline|AIMoveTimeline PlayFromStart)
    (:Update
      (Transformation|SetActorLocation (Math|Vector|Lerp(Vector) (Variables|/Game/Blueprints/BP/AI/BP_WaterAIEventTrigger.BP_WaterAIEventTrigger_C|GetStartPosition _current_event_trigger_2) (Variables|/Game/Blueprints/BP/AI/BP_WaterAIEventTrigger.BP_WaterAIEventTrigger_C|GetEndPosition _current_event_trigger_2) _alpha) false false))
    (:Finished
      (Development|PrintString (Utilities|String|ToString(Vector) (Transformation|GetActorLocation)))
      (Components|Activation|Deactivate (Variables|Default|GetParticelBody)))))

(event EventBeginPlay)

(event Collision|EventActorBeginOverlap
  (params (OtherActor :type Actor%20Object%20Reference)))

(event EventTick
  (params (DeltaSeconds :type Float%20%28single-precision%29)))

(fn ConstructionScript)