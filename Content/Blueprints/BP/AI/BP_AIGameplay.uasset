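; AI gameplay Blueprint that moves groups of stone and deck actors back and forth while the current event trigger reports IsInBox.
; Each event stores start locations and rolls random signed offsets: vertical for stones, local sideways for decks.
; Timelines lerp the actors out, reverse after a pause, then re-enter the event with new offsets.
; Movement is divided by WaterCollision's NumberOfFalls, so more falls mean smaller motion.
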(event Custom|AI%20Deck%20Event
  (bind _vectoroffsetdeck (Variables|Default|GetVectorOffsetDeck))
  ;[0.15 0.15 0.15 0.5] Setting up everything for DECK for the animation (StartLocations and VectorOffset)
  (if (Variables|/Game/Blueprints/BP/AI/BP_AIGameplayEventTrigger.BP_AIGameplayEventTrigger_C|GetIsInBox (Variables|Default|GetCurrent%20Event%20Trigger))
    (for _array_element (Variables|Default|GetDecks%20To%20Move)
      (Utilities|Array|Add (Variables|Default|GetStartLocationsDeck) (Transformation|GetActorLocation _array_element))
      (switch int (Math|Random|RandomIntegerinRange 0 1)
        (:Default
          (Utilities|Array|Add _vectoroffsetdeck (Math|Vector|MakeVector 0.0 (* (Math|Random|RandomFloatinRange 3e+02 8e+02) -1.0) 0.0) :!label _label))
        (:0
          (Utilities|Array|Add _vectoroffsetdeck (Math|Vector|MakeVector 0.0 (Math|Random|RandomFloatinRange 3e+02 8e+02) 0.0)))
        (:1
          (goto _label))))
    (Utilities|FlowControl|Delay 1.0)
    (CallFunction|PlayDeckTimeline)))

(event Custom|AI%20Stone%20Event
  (bind _vectoroffsetstone (Variables|Default|GetVectorOffsetStone))
  ;[0.15 0.15 0.15 0.5] Setting up everything for STONE for animation (StartLocation and VectorOffset)
  (if (Variables|/Game/Blueprints/BP/AI/BP_AIGameplayEventTrigger.BP_AIGameplayEventTrigger_C|GetIsInBox (Variables|Default|GetCurrent%20Event%20Trigger))
    (for _array_element (Variables|Default|GetStones%20To%20Move)
      (Utilities|Array|Add (Variables|Default|GetStartLocationsStone) (Transformation|GetActorLocation _array_element))
      (switch int (Math|Random|RandomIntegerinRange 0 1)
        (:Default
          (Utilities|Array|Add _vectoroffsetstone (Math|Vector|MakeVector 0.0 0.0 (* (Math|Random|RandomFloatinRange 3e+02 6e+02) -1.0)) :!label _label))
        (:0
          (Utilities|Array|Add _vectoroffsetstone (Math|Vector|MakeVector 0.0 0.0 (Math|Random|RandomFloatinRange 3e+02 6e+02))))
        (:1
          (goto _label))))
    (CallFunction|PlayStoneTimeline)))

(event Custom|Play%20Stone%20Timeline
  (params (Target :type Actor%20Object%20Reference) (Index :type Integer))
  ;[0.15 0.15 0.15 0.5] The animation for the Mesh
  (bind (_direction _alpha) (Timeline|Timeline_0 PlayFromStart)
    (:Update
      (for (_array_element _array_index) (Variables|Default|GetStones%20To%20Move)
        (Transformation|SetActorRelativeLocation _array_element (Math|Vector|Lerp(Vector) (Utilities|Array|Get(acopy) (Variables|Default|GetStartLocationsStone) _array_index) (+ (Utilities|Array|Get(acopy) (Variables|Default|GetVectorOffsetStone) _array_index) (Utilities|Array|Get(acopy) (Variables|Default|GetStartLocationsStone) _array_index)) (* _alpha (/ 1.0 (Math|Conversions|ToFloat(Integer) (Variables|/Game/Blueprints/BP/PlayerRespawn/BP_ResetZone.BP_ResetZone_C|GetNumber%20of%20Falls (Variables|Default|GetWaterCollision)))))))))
    (:Finished
      (switch Utilities|FlowControl|Switch|SwitchonETimelineDirection _direction
        (:Forward
          (Utilities|FlowControl|Delay 1.0)
          (CallFunction|PlayReversedStone))
        (:Backward
          (Utilities|FlowControl|Delay 2.0)
          (Utilities|Array|Clear (Variables|Default|GetVectorOffsetStone))
          (CallFunction|AIStoneEvent))))))

(event Custom|Play%20Reversed%20Stone
  ;[0.15 0.15 0.15 0.5] The animation for the Mesh
  (bind (_direction _alpha) (Timeline|Timeline_0 Reverse)
    (:Update
      (for (_array_element _array_index) (Variables|Default|GetStones%20To%20Move)
        (Transformation|SetActorRelativeLocation _array_element (Math|Vector|Lerp(Vector) (Utilities|Array|Get(acopy) (Variables|Default|GetStartLocationsStone) _array_index) (+ (Utilities|Array|Get(acopy) (Variables|Default|GetVectorOffsetStone) _array_index) (Utilities|Array|Get(acopy) (Variables|Default|GetStartLocationsStone) _array_index)) (* _alpha (/ 1.0 (Math|Conversions|ToFloat(Integer) (Variables|/Game/Blueprints/BP/PlayerRespawn/BP_ResetZone.BP_ResetZone_C|GetNumber%20of%20Falls (Variables|Default|GetWaterCollision)))))))))
    (:Finished
      (switch Utilities|FlowControl|Switch|SwitchonETimelineDirection _direction
        (:Forward
          (Utilities|FlowControl|Delay 1.0)
          (CallFunction|PlayReversedStone))
        (:Backward
          (Utilities|FlowControl|Delay 2.0)
          (Utilities|Array|Clear (Variables|Default|GetVectorOffsetStone))
          (CallFunction|AIStoneEvent))))))

(event Custom|Play%20Deck%20Timeline
  (params (Target :type Actor%20Object%20Reference) (Index :type Integer))
  ;[0.15 0.15 0.15 0.5] The animation for the Mesh
  (bind (_direction _alpha) (Timeline|Timeline PlayFromStart)
    (:Update
      (for (_array_element _array_index) (Variables|Default|GetDecks%20To%20Move)
        (Transformation|SetActorLocation _array_element (Math|Vector|Lerp(Vector) (Utilities|Array|Get(acopy) (Variables|Default|GetStartLocationsDeck) _array_index) (+ (Math|Vector|RotateVector (Utilities|Array|Get(acopy) (Variables|Default|GetVectorOffsetDeck) _array_index) (Transformation|GetActorRotation _array_element)) (Utilities|Array|Get(acopy) (Variables|Default|GetStartLocationsDeck) _array_index)) (* _alpha (/ 1.0 (Math|Conversions|ToFloat(Integer) (Variables|/Game/Blueprints/BP/PlayerRespawn/BP_ResetZone.BP_ResetZone_C|GetNumber%20of%20Falls (Variables|Default|GetWaterCollision)))))) false false)))
    (:Finished
      (switch Utilities|FlowControl|Switch|SwitchonETimelineDirection _direction
        (:Forward
          (Utilities|FlowControl|Delay 1.0)
          (CallFunction|PlayReversedDeck))
        (:Backward
          (Utilities|FlowControl|Delay 2.0)
          (Utilities|Array|Clear (Variables|Default|GetVectorOffsetDeck))
          (CallFunction|AIDeckEvent))))))

(event Custom|Play%20Reversed%20Deck
  ;[0.15 0.15 0.15 0.5] The animation for the Mesh
  (bind (_direction _alpha) (Timeline|Timeline Reverse)
    (:Update
      (for (_array_element _array_index) (Variables|Default|GetDecks%20To%20Move)
        (Transformation|SetActorLocation _array_element (Math|Vector|Lerp(Vector) (Utilities|Array|Get(acopy) (Variables|Default|GetStartLocationsDeck) _array_index) (+ (Math|Vector|RotateVector (Utilities|Array|Get(acopy) (Variables|Default|GetVectorOffsetDeck) _array_index) (Transformation|GetActorRotation _array_element)) (Utilities|Array|Get(acopy) (Variables|Default|GetStartLocationsDeck) _array_index)) (* _alpha (/ 1.0 (Math|Conversions|ToFloat(Integer) (Variables|/Game/Blueprints/BP/PlayerRespawn/BP_ResetZone.BP_ResetZone_C|GetNumber%20of%20Falls (Variables|Default|GetWaterCollision)))))) false false)))
    (:Finished
      (switch Utilities|FlowControl|Switch|SwitchonETimelineDirection _direction
        (:Forward
          (Utilities|FlowControl|Delay 1.0)
          (CallFunction|PlayReversedDeck))
        (:Backward
          (Utilities|FlowControl|Delay 2.0)
          (Utilities|Array|Clear (Variables|Default|GetVectorOffsetDeck))
          (CallFunction|AIDeckEvent))))))

(event EventBeginPlay)

(event Collision|EventActorBeginOverlap
  (params (OtherActor :type Actor%20Object%20Reference)))

(event EventTick
  (params (DeltaSeconds :type Float%20%28single-precision%29)))

(fn ConstructionScript)