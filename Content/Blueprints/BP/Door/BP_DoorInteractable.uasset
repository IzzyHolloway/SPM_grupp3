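; BP_DoorInteractable is an interactable door that teleports the player between inside and outside positions.
; On interact, a guard flag blocks re-entry while a black fade widget and door sound play.
; The BP_CameraDirector's active zone decides the direction and switches to the destination zone; only exiting also moves the camera director.
; After a one-second delay it removes the fade, clears the guard and marks the character's camera instructions as shown.
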(event EventBeginPlay)

(event Collision|EventActorBeginOverlap
  (params (OtherActor :type Actor%20Object%20Reference)))

(event EventTick
  (params (DeltaSeconds :type Float%20%28single-precision%29)))

(event EventOnDoorInteract
  (bind _returnvalue (Game|GetPlayerCharacter 0))
  (if (not (Variables|Default|GetbIsGoingThruDoor))
    (Variables|Default|SetbIsGoingThruDoor true)
    (bind _returnvalue_2 (UserInterface|CreateWidget "/Game/Blueprints/WBP/Loading/WBP_BlackFade.WBP_BlackFade_C"))
    (UserInterface|Viewport|AddtoViewport _returnvalue_2 0)
    (Audio|PlaySound2D "/Game/Grupp03_Test/Zoey/Audio/Door/SC_SFX_Door.SC_SFX_Door" 1.0 1.0 0.0 0 0)
    (Default|FadeScreen _returnvalue_2 true)
    (bind _returnvalue_3 (Actor|GetActorOfClass "/Game/Blueprints/BP/Camera/BP_CameraDirector.BP_CameraDirector_C"))
    (if (Variables|/Game/Blueprints/BP/Camera/BP_CameraZone.BP_CameraZone_C|GetIsInside (Variables|/Game/Blueprints/BP/Camera/BP_CameraDirector.BP_CameraDirector_C|GetActiveZone _returnvalue_3))
      (Transformation|SetActorLocation _returnvalue (Variables|Default|GetOutsidePosition) false true)
      (bind _returnvalue_4 (Actor|GetActorOfClass "/Game/Blueprints/BP/Camera/BP_CameraDirector.BP_CameraDirector_C"))
      (bind _output_get (Variables|/Game/Blueprints/BP/Camera/BP_CameraDirector.BP_CameraDirector_C|SetActiveZone _returnvalue_4 (Variables|Default|GetOutsideZone)))
      (Transformation|SetActorLocation _returnvalue_4 (+ (Variables|/Game/Blueprints/BP/Camera/BP_CameraZone.BP_CameraZone_C|GetCameraOffset _output_get) (Variables|Default|GetOutsidePosition)) false true)
      (else
        (Transformation|SetActorLocation _returnvalue (Variables|Default|GetInsidePosition) false true)
        (bind _returnvalue_5 (Actor|GetActorOfClass "/Game/Blueprints/BP/Camera/BP_CameraDirector.BP_CameraDirector_C"))
        (Variables|/Game/Blueprints/BP/Camera/BP_CameraDirector.BP_CameraDirector_C|SetActiveZone _returnvalue_5 (Variables|Default|GetInsideZone))))
    (Utilities|FlowControl|Delay 1.0)
    (Default|FadeScreen _returnvalue_2 false)
    (Widget|RemovefromParent _returnvalue_2)
    (Variables|Default|SetbIsGoingThruDoor false)
    (bind _returnvalue_6 (Actor|GetActorOfClass "/Game/Characters/BP_CharacterSpeltest1.BP_CharacterSpeltest1_C"))
    (Variables|/Game/Characters/BP_CharacterSpeltest1.BP_CharacterSpeltest1_C|SetbHasShownCameraInstructions _returnvalue_6 true)))

(fn ConstructionScript)