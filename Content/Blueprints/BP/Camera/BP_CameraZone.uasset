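; BP_CameraZone is a trigger volume that registers itself as the active zone on the BP_CameraDirector.
; On BeginPlay it waits briefly, then sets the director's ActiveZone to itself.
; When a BP_CharacterSpeltest1 actor enters its TriggerBox, it claims ActiveZone again, unless BP_Boat_Functionality is possessed.
; Director and boat are both looked up at runtime with GetActorOfClass.
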(event OnComponentBeginOverlap(TriggerBox)
  (params (OverlappedComponent :type Primitive%20Component%20Object%20Reference) (OtherActor :type Actor%20Object%20Reference) (OtherComp :type Primitive%20Component%20Object%20Reference) (OtherBodyIndex :type Integer) (bFromSweep :type Boolean) (SweepResult :type Hit%20Result%20Structure%20%28by%20ref%29))
  (if (Utilities|ClassIsChildOf (Utilities|GetClass OtherActor) "/Game/Characters/BP_CharacterSpeltest1.BP_CharacterSpeltest1_C")
    (bind _returnvalue (Actor|GetActorOfClass "/Game/Blueprints/BP/Boat/BP_Boat_Functionality.BP_Boat_Functionality_C"))
    (if (not (Variables|/Game/Blueprints/BP/Boat/BP_Boat_Functionality.BP_Boat_Functionality_C|GetPossessed _returnvalue))
      (bind _returnvalue_2 (Actor|GetActorOfClass "/Game/Blueprints/BP/Camera/BP_CameraDirector.BP_CameraDirector_C"))
      (Variables|/Game/Blueprints/BP/Camera/BP_CameraDirector.BP_CameraDirector_C|SetActiveZone _returnvalue_2 self))))

(event EventBeginPlay
  (Utilities|FlowControl|Delay 0.2)
  (bind _returnvalue (Actor|GetActorOfClass "/Game/Blueprints/BP/Camera/BP_CameraDirector.BP_CameraDirector_C"))
  (Variables|/Game/Blueprints/BP/Camera/BP_CameraDirector.BP_CameraDirector_C|SetActiveZone _returnvalue self))

(event Collision|EventActorBeginOverlap
  (params (OtherActor :type Actor%20Object%20Reference)))

(event EventTick
  (params (DeltaSeconds :type Float%20%28single-precision%29)))

(fn ConstructionScript)