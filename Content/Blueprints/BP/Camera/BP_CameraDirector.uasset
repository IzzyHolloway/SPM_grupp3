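; Camera director actor that becomes the player's view target behind a black fade and drives both gameplay framing and cutscenes.
; Tick runs any flagged cutscene (islands, lighthouse, entity), otherwise frames by the active BP_CameraZone: follow with dock/boat midpoint, fixed room or vertical follow.
; Cutscenes end on delays or dialogue-manager callbacks, with some lowering island fog.
; Control yaw eases to the zone's camera, and the dialogue-advance input drives hold-to-skip.
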(event Custom|Play%20Cutscene%201
  (bind _island1fog (Variables|Default|GetIsland1Fog))
  (bind _returnvalue (Transformation|GetActorLocation _island1fog))
  (bind (_x _y _z) (Math|Vector|BreakVector _returnvalue))
  ;[0.15 0.15 0.15 0.5] Cutscenes for the camera.
  (Transformation|SetActorLocation (Math|Interpolation|VInterpTo (Transformation|GetActorLocation) (Variables|Default|GetIsland1CutsceneLocation) (Utilities|Time|GetWorldDeltaSeconds) 2.0) false false)
  (Transformation|SetActorRotation (Math|Interpolation|RInterpTo (Transformation|GetActorRotation) (Variables|Default|GetIsland1CutsceneRotation) (Utilities|Time|GetWorldDeltaSeconds) 2.0))
  (Transformation|SetActorLocation _island1fog (Math|Interpolation|VInterpTo _returnvalue (Math|Vector|MakeVector _x _y (- _z 1e+04)) (Utilities|Time|GetWorldDeltaSeconds) 2.0) false false)
  (Utilities|FlowControl|Delay 7.0)
  (Variables|Default|SetbIsInCutscene1 false)
  (bind _returnvalue_2 (Actor|GetActorOfClass "/Game/Characters/BP_CharacterSpeltest1.BP_CharacterSpeltest1_C"))
  (Class|CharacterAimi|SetMovementLocked _returnvalue_2 false))

(event Custom|PanBackCameraRotation
  ;[0.15 0.15 0.15 0.5] Place camera back to its original rotation
  (Transformation|SetActorRotation (Math|Rotator|Lerp(Rotator) (Transformation|GetActorRotation self) (Variables|/Game/Blueprints/BP/Camera/BP_CameraZone.BP_CameraZone_C|GetCameraRotation (Variables|Default|GetActiveZone)) 0.0)))

(event Custom|Entit%20Cutscene%20End
  ;[0.15 0.15 0.15 0.5] Cutscenes for the camera.
  (Variables|Default|SetbIsInEntityCutscene false))

(event Custom|Entity%20cutscene
  ;[0.15 0.15 0.15 0.5] Cutscenes for the camera.
  (Transformation|SetActorLocation (Math|Interpolation|VInterpTo (Transformation|GetActorLocation) (Variables|Default|GetEntityCameraLocation) (Utilities|Time|GetWorldDeltaSeconds) 2.0) false false)
  (Transformation|SetActorRotation (Math|Interpolation|RInterpTo (Transformation|GetActorRotation) (Variables|Default|GetEntityCameraRotation) (Utilities|Time|GetWorldDeltaSeconds) 2.0))
  (bind _returnvalue (Actor|GetActorOfClass "/Game/Blueprints/BP/Managers/BP_DialogueManager.BP_DialogueManager_C"))
  (EventDispatchers|BindEventtoOnDialogueEnded _returnvalue (delegate Custom|Entit%20Cutscene%20End)))

(event Custom|Island%202%20Cutscene%20End
  ;[0.15 0.15 0.15 0.5] Cutscenes for the camera.
  (Variables|Default|SetbIsInCutscene2 false))

(event Custom|Play%20Cutscene%202
  ;[0.15 0.15 0.15 0.5] Cutscenes for the camera.
  (Transformation|SetActorLocation (Math|Interpolation|VInterpTo (Transformation|GetActorLocation) (Variables|Default|GetIsland2CutsceneLocation) (Utilities|Time|GetWorldDeltaSeconds) 2.0) false false)
  (Transformation|SetActorRotation (Math|Interpolation|RInterpTo (Transformation|GetActorRotation) (Variables|Default|GetIsland2CutsceneRotation) (Utilities|Time|GetWorldDeltaSeconds) 2.0))
  (bind _returnvalue (Actor|GetActorOfClass "/Game/Blueprints/BP/Managers/BP_DialogueManager.BP_DialogueManager_C"))
  (EventDispatchers|BindEventtoOnDialogueEnded _returnvalue (delegate Custom|Island%202%20Cutscene%20End)))

(event Custom|PlayLighthouseCutscene
  ;[0.15 0.15 0.15 0.5] Cutscenes for the camera.
  (Variables|Default|SetbIsInCutsceneLighthouse true)
  (Transformation|SetActorLocation (Utilities|Array|Get(acopy) (Variables|Default|GetIslandLighthouseLocation) (Variables|Default|GetCurrentIndex)) false true)
  (Transformation|SetActorRotation (Utilities|Array|Get(acopy) (Variables|Default|GetIslandLighthouseRotation) (Variables|Default|GetCurrentIndex)) true)
  (Utilities|FlowControl|Delay 4.0)
  (Math|Integer|IncrementInt (Variables|Default|GetCurrentIndex)
    (:%20%20
      (if (> (Variables|Default|GetCurrentIndex) 2)
        (Variables|Default|SetCurrentIndex 2))
      (bind _returnvalue (Actor|GetActorOfClass "/Game/Blueprints/BP/Managers/BP_DialogueManager.BP_DialogueManager_C"))
      (EventDispatchers|BindEventtoOnDialogueEnded _returnvalue (delegate Custom|LighthouseCutsceneEnd)))))

(event Custom|Play%20Cutscene%203
  (bind _island2fog (Variables|Default|GetIsland2Fog))
  (bind _returnvalue (Transformation|GetActorLocation _island2fog))
  (bind (_x _y _z) (Math|Vector|BreakVector _returnvalue))
  ;[0.15 0.15 0.15 0.5] Cutscenes for the camera.
  (Transformation|SetActorLocation (Math|Interpolation|VInterpTo (Transformation|GetActorLocation) (Variables|Default|GetIsland2EndCutsceneLocation) (Utilities|Time|GetWorldDeltaSeconds) 2.0) false false)
  (Transformation|SetActorRotation (Math|Interpolation|RInterpTo (Transformation|GetActorRotation) (Variables|Default|GetIsland2EndCutsceneRotation') (Utilities|Time|GetWorldDeltaSeconds) 2.0))
  (Transformation|SetActorLocation _island2fog (Math|Interpolation|VInterpTo _returnvalue (Math|Vector|MakeVector _x _y (- _z 1e+04)) (Utilities|Time|GetWorldDeltaSeconds) 2.0) false false)
  (Utilities|FlowControl|Delay 7.0)
  (Variables|Default|SetbIsInCutscene3 false)
  (bind _returnvalue_2 (Actor|GetActorOfClass "/Game/Characters/BP_CharacterSpeltest1.BP_CharacterSpeltest1_C"))
  (Class|CharacterAimi|SetMovementLocked _returnvalue_2 false))

(event Custom|LighthouseCutsceneEnd
  ;[0.15 0.15 0.15 0.5] Cutscenes for the camera.
  (Variables|Default|SetbIsInCutsceneLighthouse false))

(event Input|EnhancedActionEvents|EnhancedInputActionIA_DialogueAdvance
  (params (ActionValue :type Boolean) (ElapsedSeconds :type Float%20%28double-precision%29) (TriggeredSeconds :type Float%20%28double-precision%29) (InputAction :type Input%20Action%20Object%20Reference :default "/Game/Input/Actions/IA_DialogueAdvance.IA_DialogueAdvance"))
  (bind _skippromptwidget (Variables|Default|GetSkipPromptWidget))
  (bind _skippromptwidget_2 (Variables|Default|GetSkipPromptWidget))
  (:Started
    (if (Variables|Default|GetbCutsceneActive)
      (Utilities|IsValid _skippromptwidget
        (:Is%20Valid
          (Default|StartSkipHold _skippromptwidget)))))
  (:Canceled
    (if (Variables|Default|GetbCutsceneActive) :!label _label
      (Utilities|IsValid _skippromptwidget_2
        (:Is%20Valid
          (Default|StopSkipHold _skippromptwidget_2)))))
  (:Completed
    (goto _label)))

(event EventBeginPlay
  ;[0.15 0.15 0.15 0.5] Set player view
  (bind _returnvalue (UserInterface|CreateWidget "/Game/Blueprints/WBP/TransitionScenes/WBP_BlackFade.WBP_BlackFade_C"))
  (UserInterface|Viewport|AddtoViewport _returnvalue 0)
  (Default|FadeScreen _returnvalue true)
  (Utilities|FlowControl|DelayUntilNextFrame)
  (Input|EnableInput self (Game|GetPlayerController 0))
  (Utilities|IsValid (Pawn|GetControlledPawn (Game|GetPlayerController 0))
    (:Is%20Valid
      (Game|Player|SetViewTargetwithBlend (Game|GetPlayerController 0) self 0.0 "VTBlend_Linear" 0.0 false)
      (Utilities|FlowControl|Delay 1.5)
      (Variables|Default|SetActiveZone (Utilities|Array|Get(acopy) (Collision|GetOverlappingActors (Game|GetPlayerCharacter 0) "/Game/Blueprints/BP/Camera/BP_CameraZone.BP_CameraZone_C" :!class /Script/Engine.Actor)))
      (Default|FadeScreen _returnvalue false)
      (Widget|RemovefromParent _returnvalue))))

(event Collision|EventActorBeginOverlap
  (params (OtherActor :type Actor%20Object%20Reference)))

(event EventTick
  (params (DeltaSeconds :type Float%20%28single-precision%29))
  (bind _returnvalue (Game|GetPlayerCharacter 0))
  (bind _activezone (Variables|Default|GetActiveZone))
  (bind _cinecamera (Variables|Default|GetCineCamera))
  (bind _activezone_2 (Variables|Default|GetActiveZone))
  (bind _activezone_3 (Variables|Default|GetActiveZone))
  (bind _activezone_4 (Variables|Default|GetActiveZone))
  (bind _returnvalue_2 (Transformation|GetActorLocation _returnvalue))
  (bind _returnvalue_3 (Transformation|GetActorLocation _activezone_4))
  (bind _relateddoor (Variables|/Game/Blueprints/BP/Camera/BP_CameraZone.BP_CameraZone_C|GetRelatedDoor _activezone_3))
  (bind (_x _y) (Math|Vector|BreakVector _returnvalue_3))
  (if (Utilities|IsValid _activezone)
    (if (Variables|Default|GetbIsInCutscene1)
      (CallFunction|PlayCutscene1)
      (elif (Variables|Default|GetbIsInCutscene2)
        (CallFunction|PlayCutscene2)
        (elif (Variables|Default|GetbIsInCutscene3)
          (CallFunction|PlayCutscene3)
          (elif (Variables|Default|GetbIsInCutsceneLighthouse)
            (CallFunction|PlayLighthouseCutscene)
            (elif (Variables|Default|GetbIsInEntityCutscene)
              (CallFunction|EntityCutscene)
              (else
                (switch Utilities|FlowControl|Switch|SwitchonE_CameraBehaviour (Variables|/Game/Blueprints/BP/Camera/BP_CameraZone.BP_CameraZone_C|GetCameraZoneBehaviour _activezone)
                  (:NewEnumerator0
                    (if (Utilities|IsValid _returnvalue)
                      (if (Variables|/Game/Blueprints/BP/Camera/BP_CameraZone.BP_CameraZone_C|GetIsAtDock (Variables|Default|GetActiveZone))
                        ;[0.15 0.15 0.15 0.5] Adjusting Camera location if at dock
                        (bind _returnvalue_4 (CallFunction|FindCameraLocation _returnvalue_2 (Transformation|GetActorLocation (Variables|Default|GetBoatReference)) 2.0))
                        (Transformation|SetActorLocation _returnvalue_4 false false)
                        (Class|PlayerCameraManager|SetGameCameraCutThisFrame (Variables|/Script/Engine.PlayerController|GetPlayerCameraManager (Game|GetPlayerController (Variables|/Script/Engine.Pawn|GetPlayerState (Game|GetPlayerCharacter 0)))))
                        (else
                          ;[0.15 0.15 0.15 0.5] Handle the camera outside
                          (bind _returnvalue_5 (CallFunction|FindCameraLocation _returnvalue_2 "0, 0, 0" 1.0))
                          (Transformation|SetActorLocation _returnvalue_5 false false)
                          (Class|PlayerCameraManager|SetGameCameraCutThisFrame (Variables|/Script/Engine.PlayerController|GetPlayerCameraManager (Game|GetPlayerController (Variables|/Script/Engine.Pawn|GetPlayerState (Game|GetPlayerCharacter 0)))))))
                      (bind _returnvalue_6 (CallFunction|FindCameraRotation (Utilities|Time|GetWorldDeltaSeconds)))
                      (Transformation|SetActorRotation _returnvalue_6)
                      (Transformation|SetRelativeRotation _cinecamera (Math|Interpolation|RInterpTo (Variables|/Script/Engine.SceneComponent|GetRelativeRotation _cinecamera) (Variables|Default|GetPlayerRotationOffset) (Utilities|Time|GetWorldDeltaSeconds) 2.0) false false)
                      (CallFunction|AdjustPlayerControlRotation)))
                  (:NewEnumerator1
                    ;[0.15 0.15 0.15 0.5] Handles the fixed camera inside
                    (if (Utilities|IsValid _relateddoor)
                      (Transformation|SetActorLocation (+ (Variables|/Game/Blueprints/BP/Level_Interactions/BP_DoorInteractable.BP_DoorInteractable_C|GetInsidePosition _relateddoor) (Variables|/Game/Blueprints/BP/Camera/BP_CameraZone.BP_CameraZone_C|GetCameraOffset _activezone_2)) false true)
                      (Transformation|SetActorRelativeRotation self (Variables|/Game/Blueprints/BP/Camera/BP_CameraZone.BP_CameraZone_C|GetCameraRotation _activezone_2))
                      (CallFunction|AdjustPlayerControlRotation)))
                  (:NewEnumerator2
                    (Transformation|SetActorLocation (Math|Interpolation|VInterpTo (Transformation|GetActorLocation) (+ (Variables|/Game/Blueprints/BP/Camera/BP_CameraZone.BP_CameraZone_C|GetCameraOffset _activezone_4) (Math|Vector|MakeVector _x _y (Math|Float|Clamp(Float) (.Z (Math|Vector|BreakVector (Transformation|GetActorLocation (Game|GetPlayerCharacter 0)))) 0.0 4219.489943))) (Utilities|Time|GetWorldDeltaSeconds) 2.0) false false)
                    (Transformation|SetActorRotation (Variables|/Game/Blueprints/BP/Camera/BP_CameraZone.BP_CameraZone_C|GetCameraRotation (Variables|Default|GetActiveZone)))
                    (CallFunction|AdjustPlayerControlRotation)))))))))))

(fn ConstructionScript)

(fn FindCameraLocation
  (params (A :type Vector) (B :type Vector) (Actors :type Float%20%28double-precision%29))
  (if (Utilities|IsValid (Variables|Default|GetActiveZone))
    (return (Math|Interpolation|VInterpTo (Transformation|GetActorLocation self) (+ (/ (+ A B) Actors) (Variables|/Game/Blueprints/BP/Camera/BP_CameraZone.BP_CameraZone_C|GetCameraOffset (Variables|Default|GetActiveZone))) (Utilities|Time|GetWorldDeltaSeconds) 2.0))
    (else
      (return "0, 0, 0"))))

(fn FindCameraRotation
  (params (DeltaTime :type Float%20%28single-precision%29))
  (if (Utilities|IsValid (Variables|Default|GetActiveZone))
    (return (Math|Interpolation|RInterpTo (Transformation|GetActorRotation self) (Variables|/Game/Blueprints/BP/Camera/BP_CameraZone.BP_CameraZone_C|GetCameraRotation (Variables|Default|GetActiveZone)) DeltaTime 2.0))))

(fn SplineProgressCalculation
  (params (Input :type Float%20%28double-precision%29))
  (return (+ (Variables|Default|GetSplineProgress) (* Input (Variables|/Game/Blueprints/BP/Camera/BP_CameraZone.BP_CameraZone_C|GetTransitionSpeed (Variables|Default|GetActiveZone))))))

(fn AdjustPlayerControlRotation
  (bind _returnvalue (Game|GetPlayerController 0))
  (Pawn|SetControlRotation _returnvalue (Math|Interpolation|RInterpTo (Pawn|GetControlRotation _returnvalue :!class /Script/Engine.Controller) (Math|Rotator|MakeRotator 0.0 0.0 (.Yaw (Math|Rotator|BreakRotator (Variables|/Game/Blueprints/BP/Camera/BP_CameraZone.BP_CameraZone_C|GetCameraRotation (Variables|Default|GetActiveZone))))) (Utilities|Time|GetWorldDeltaSeconds) 2.0))
  (return))