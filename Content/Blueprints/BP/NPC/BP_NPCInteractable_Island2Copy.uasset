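; Island 2 NPC that walks along splines to a door, later walks out of the house, then flags itself as dancing.
; MoveToDoor starts the first spline walk, while the ProgressionManager flag "Island2NPCExitedHouse" triggers the second, checked on BeginPlay and polled each Tick until set.
; Tick advances distance by speed, setting location and yaw from splines cached in the Construction Script.
; Collision stays off until the exit walk begins.
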(event Custom|MoveToDoor
  ;[0.15 0.15 0.15 0.5] Start walking to the door
  (Variables|Default|SetIsWalkingToDoor true))

(event EventTick
  (params (DeltaSeconds :type Float%20%28single-precision%29))
  (if (Variables|Default|GetHasStartedExit)
    ;[0.15 0.15 0.15 0.5] 2. Walk out of the house
    (if (Variables|Default|GetIsWalkingOutOfHouse)
      (Collision|SetActorEnableCollision true)
      (CallFunction|MoveandRotateAlongSpline DeltaSeconds (Variables|Default|GetSplinePart2))
      ;[0.15 0.15 0.15 0.5] End walking if whole distances has been travelled and start dance animation
      (bind _returnvalue (CallFunction|HasWholeDistanceBeenTravelled (Variables|Default|GetSplinePart2)))
      (if _returnvalue
        (Variables|Default|SetIsWalkingOutOfHouse false)
        (Variables|Default|SetIsDancing true)))
    (else
      (Utilities|FlowControl|Sequence
        (:then_0
          ;[0.15 0.15 0.15 0.5] 1. Walk to the door
          (if (Variables|Default|GetIsWalkingToDoor)
            (CallFunction|MoveandRotateAlongSpline DeltaSeconds (Variables|Default|GetSplinePart1))
            ;[0.15 0.15 0.15 0.5] End walking if whole distances has been travelled
            (bind _returnvalue_2 (CallFunction|HasWholeDistanceBeenTravelled (Variables|Default|GetSplinePart1)))
            (if _returnvalue_2
              (Variables|Default|SetIsWalkingToDoor false)
              ;;[0.15 0.15 0.15 0.5] Reset distance for walking along another spline later
              (Variables|Default|SetCurrentDistance 0.0))))
        (:then_1
          ;[0.15 0.15 0.15 0.5] Progression
          (bind _returnvalue_3 (Actor|GetActorOfClass "/Script/SPM_grupp3.ProgressionManager"))
          (if (Class|ProgressionManager|HasFlag _returnvalue_3 "Island2NPCExitedHouse")
            (Variables|Default|SetIsWalkingOutOfHouse true)
            (Variables|Default|SetHasStartedExit true)))))))

(event EventBeginPlay
  ;[0.15 0.15 0.15 0.5] Progression
  (Collision|SetActorEnableCollision false)
  (bind _returnvalue (Actor|GetActorOfClass "/Script/SPM_grupp3.ProgressionManager"))
  (if (Class|ProgressionManager|HasFlag _returnvalue "Island2NPCExitedHouse")
    (Variables|Default|SetIsWalkingOutOfHouse true)
    (Variables|Default|SetHasStartedExit true)
    (else
      (Variables|Default|SetIsWalkingOutOfHouse false)
      (Variables|Default|SetHasStartedExit false))))

(fn ConstructionScript
  ;[0.15 0.15 0.15 0.5] Save spline components of spline actors
  (Variables|Default|SetSplinePart2 (Actor|GetComponentbyClass (Variables|Default|GetSplineActorPart2) "/Script/Engine.SplineComponent"))
  (Variables|Default|SetSplinePart1 (Actor|GetComponentbyClass (Variables|Default|GetSplineActorPart1) "/Script/Engine.SplineComponent")))

(fn MoveandRotateAlongSpline
  (params (DeltaSeconds :type Float%20%28double-precision%29) (Spline :type Spline%20Component%20Object%20Reference))
  ;[0.15 0.15 0.15 0.5] Update current distance: Add distance walked this frame
  (Variables|Default|SetCurrentDistance (+ (Variables|Default|GetCurrentDistance) (* (Variables|Default|GetSpeed) DeltaSeconds)))
  ;[0.15 0.15 0.15 0.5] Set new actor location: distance along spline
  (Transformation|SetActorLocation (Spline|GetLocationatDistanceAlongSpline Spline (Variables|Default|GetCurrentDistance) "World") false false)
  ;[0.15 0.15 0.15 0.5] Set new rotation: Not needed right now, since NPC looks the same from all sides
  (Transformation|SetActorRotation (Math|Rotator|MakeRotator 0.0 0.0 (- (.yaw (Spline|GetRotationatDistanceAlongSpline Spline (Variables|Default|GetCurrentDistance) "Local")) 9e+01))))

(fn HasWholeDistanceBeenTravelled
  (params (Spline :type Spline%20Component%20Object%20Reference))
  (return (>= (Variables|Default|GetCurrentDistance) (Spline|GetSplineLength Spline))))