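; Trigger box actor that plays intro dialogue once when BP_CharacterSpeltest1 enters, then sends TargetNPC to a door on the first end overlap.
; Island booleans select which BP_CameraDirector cutscene flag to raise before BP_DialogueManager starts the first dialogue entry, optionally with a completion flag.
; The unflagged path clears IsInCutscene1 right after starting dialogue.
; After a one-second startup delay, it destroys itself if BP_ProgressionManager already holds that flag.
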(event OnComponentBeginOverlap(Box)
  (params (OverlappedComponent :type Primitive%20Component%20Object%20Reference) (OtherActor :type Actor%20Object%20Reference) (OtherComp :type Primitive%20Component%20Object%20Reference) (OtherBodyIndex :type Integer) (bFromSweep :type Boolean) (SweepResult :type Hit%20Result%20Structure%20%28by%20ref%29))
  (bind _introdialoguedata (Variables|Default|GetIntroDialogueData))
  (bind _dialogueentries (Variables|/Script/SPM_grupp3.DialogueDataAsset|GetDialogueEntries _introdialoguedata))
  (bind _output (Utilities|Array|Get(acopy) _dialogueentries))
  (bind (_dialogueid _requiredflags _blockedflags _dialoguelines _rawdialogueimporttext _bsetflagondialogueend _flagtosetondialogueend) (Utilities|Struct|BreakDialogueEntry _output))
  (Utilities|Casting|CastToBP_CharacterSpeltest1 OtherActor)
  (Utilities|FlowControl|DoOnce false
    (:Completed
      (if (Variables|Default|GetbIsIsland2)
        (bind _returnvalue (Actor|GetActorOfClass "/Game/Blueprints/BP/Camera/BP_CameraDirector.BP_CameraDirector_C"))
        (Variables|/Game/Blueprints/BP/Camera/BP_CameraDirector.BP_CameraDirector_C|SetbIsInCutscene2 _returnvalue true)
        (elif (Variables|Default|GetbIsLighthouseIsland)
          (bind _returnvalue_2 (Actor|GetActorOfClass "/Game/Blueprints/BP/Camera/BP_CameraDirector.BP_CameraDirector_C"))
          (Variables|/Game/Blueprints/BP/Camera/BP_CameraDirector.BP_CameraDirector_C|SetbIsInEntityCutscene _returnvalue_2 true)))
      (bind _returnvalue_3 (Actor|GetActorOfClass "/Game/Blueprints/BP/Managers/BP_DialogueManager.BP_DialogueManager_C"))
      (if _bsetflagondialogueend
        (Class|DialogueManager|StartDialoguewithFlag _returnvalue_3 _dialoguelines _flagtosetondialogueend)
        (else
          (Class|DialogueManager|StartDialogue _returnvalue_3 _dialoguelines)
          (bind _returnvalue_4 (Actor|GetActorOfClass "/Game/Blueprints/BP/Camera/BP_CameraDirector.BP_CameraDirector_C"))
          (Variables|/Game/Blueprints/BP/Camera/BP_CameraDirector.BP_CameraDirector_C|SetbIsInCutscene1 _returnvalue_4 false))))))

(event OnComponentEndOverlap(Box)
  (params (OverlappedComponent :type Primitive%20Component%20Object%20Reference) (OtherActor :type Actor%20Object%20Reference) (OtherComp :type Primitive%20Component%20Object%20Reference) (OtherBodyIndex :type Integer))
  (bind _targetnpc (Variables|Default|GetTargetNPC))
  (Utilities|FlowControl|DoOnce false
    (:Completed
      (Utilities|IsValid _targetnpc
        (:Is%20Valid
          (Default|MovetoDoor _targetnpc))))))

(event EventBeginPlay
  (Utilities|FlowControl|Delay 1.0)
  (bind _returnvalue (Actor|GetActorOfClass "/Game/Blueprints/BP/Managers/BP_ProgressionManager.BP_ProgressionManager_C"))
  (if (Class|ProgressionManager|HasFlag _returnvalue (.FlagToSetOnDialogueEnd (Utilities|Struct|BreakDialogueEntry (Utilities|Array|Get(acopy) (Variables|/Script/SPM_grupp3.DialogueDataAsset|GetDialogueEntries (Variables|Default|GetIntroDialogueData))))))
    (Actor|DestroyActor)))

(fn ConstructionScript)