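; Reset zone that returns the player character to its last saved position after it falls into the volume.
; A Box overlap filters for BP_CharacterSpeltest1, then looks up the BP_Boat_Functionality actor in the level.
; Only while that boat is not possessed does it move the character to LastSavedPosition and increment its own NumberOfFalls counter.
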(event OnComponentBeginOverlap(Box)
  (params (OverlappedComponent :type Primitive%20Component%20Object%20Reference) (OtherActor :type Actor%20Object%20Reference) (OtherComp :type Primitive%20Component%20Object%20Reference) (OtherBodyIndex :type Integer) (bFromSweep :type Boolean) (SweepResult :type Hit%20Result%20Structure%20%28by%20ref%29))
  (if (Utilities|ClassIsChildOf (Utilities|GetClass OtherActor) "/Game/Characters/BP_CharacterSpeltest1.BP_CharacterSpeltest1_C")
    (bind _asbp_character_speltest_1 (Utilities|Casting|CastToBP_CharacterSpeltest1 OtherActor))
    (bind _returnvalue (Actor|GetActorOfClass "/Game/Blueprints/BP/Boat/BP_Boat_Functionality.BP_Boat_Functionality_C"))
    (if (not (Variables|/Game/Blueprints/BP/Boat/BP_Boat_Functionality.BP_Boat_Functionality_C|GetPossessed _returnvalue))
      (Transformation|SetActorLocation _asbp_character_speltest_1 (Variables|/Game/Characters/BP_CharacterSpeltest1.BP_CharacterSpeltest1_C|GetLastSavedPosition _asbp_character_speltest_1) false false)
      (Math|Integer|IncrementInt (Variables|Default|GetNumber%20of%20Falls)))))

(event EventBeginPlay)

(event Collision|EventActorBeginOverlap
  (params (OtherActor :type Actor%20Object%20Reference)))

(event EventTick
  (params (DeltaSeconds :type Float%20%28single-precision%29)))

(fn ConstructionScript)